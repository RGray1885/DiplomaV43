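; Base NPC that can be fought, killed and talked to, with state changes passed to its AI controller's Blackboard.
; Player damage flags combat and lowers HP; death disables movement, plays a montage, drops loot, grants XP and notifies the quest log.
; A timer later resurrects it in place with full HP.
; Clicks and dialogue closing toggle the interaction key, while cursor hover toggles mesh custom depth.
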(event `self.ReceiveBeginPlay`
  (set `self.CurrentHP` (`self.MaxHP`))
  (`BlackboardComponent.SetValueAsBool` (`AIBlueprintHelperLibrary.GetBlackboard` (`AIBlueprintHelperLibrary.GetAIController` self)) "IsDead" false))

(event `self.ReceiveAnyDamage`
  (params (Damage :type "Float (single-precision)") (DamageType :type "DamageType Object Reference") (InstigatedBy :type "Controller Object Reference") (DamageCauser :type "Actor Object Reference"))
  (bind _returnvalue (`AIBlueprintHelperLibrary.GetBlackboard` (`AIBlueprintHelperLibrary.GetAIController` self)))
  (if (> (`self.CurrentHP`) 0)
    (bind _asbp_player (cast `/Game/Base/BP_Player` DamageCauser))
    (`/Game/Base/BP_Player_HUD.ShowTargetName` (`/Game/Base/BFL_BasicFunctions.Get Player HUD`) self)
    (`BlackboardComponent.SetValueAsObject` _returnvalue "Attacker" DamageCauser)
    (`BlackboardComponent.SetValueAsBool` _returnvalue "InCombat" true)
    (`KismetSystemLibrary.PrintString` (`KismetStringLibrary.BuildString_Double` (`KismetSystemLibrary.GetDisplayName` DamageCauser) "dealt " Damage " of damage"))
    (bind _output_get (set `self.CurrentHP` (- (`self.CurrentHP`) (`KismetMathLibrary.FTrunc` Damage))))
    (if (<= _output_get 0)
      (`self.PlayDead`)
      (`/Game/SubSystems/LootDrop/AC_LootDrop.DropLoot` (`self.AC_LootDrop`)))))

(event `PlayDead`
  (bind _charactermovement (`self.CharacterMovement`))
  (bind _returnvalue (`AIBlueprintHelperLibrary.GetAIController` self))
  (set `self.IsDead` true)
  (`BlackboardComponent.SetValueAsBool` (`AIController.Blackboard` _returnvalue) "IsDead" true)
  (`self.DisableInput` _returnvalue null)
  (`MovementComponent.StopMovementImmediately` _charactermovement)
  (`CharacterMovementComponent.DisableMovement` _charactermovement)
  (`|PlayMontage` (`self.Mesh`) (`self.DeathMontage`)
    (:`then`
      (`/Game/SubSystems/PlayerStats/SystemFiles/AC_CharacterStats.AddExperience` (`/Game/Base/BP_Player.PlayerStats` (stale `self.ReceiveAnyDamage` _asbp_player)) (`self.KillXP`))
      (`/Game/SubSystems/QuestSystem/SystemFiles/AC_QuestLog.OnObjectiveCalled` (`/Game/Base/BFL_BasicFunctions.GetPlayerQuestLog`) (`self.NPCType`))
      (`KismetSystemLibrary.K2_SetTimerDelegate` (delegate `Resurrect`) 10.0))))

(event `Resurrect`
  (bind _returnvalue (`AIBlueprintHelperLibrary.GetAIController` self))
  (`CharacterMovementComponent.SetMovementMode` (`self.CharacterMovement`) "MOVE_Walking" 0)
  (set `self.IsDead` false)
  (set `self.CurrentHP` (`self.MaxHP`))
  (`AnimInstance.Montage_Stop` (`SkeletalMeshComponent.GetAnimInstance` (`self.Mesh`)) 0.0 null)
  (`BlackboardComponent.SetValueAsBool` (`AIController.Blackboard` _returnvalue) "IsDead" false)
  (bind _asbp_aicontroller (cast `/Game/NPC/AI/BP_AIController` _returnvalue))
  (`/Game/NPC/AI/BP_AIController.ResetPlayerNoticed` _asbp_aicontroller))

(event `self.ReceiveActorOnClicked`
  (params (ButtonPressed :type "Key Structure"))
  (bind _asbp_aicontroller (cast `/Game/NPC/AI/BP_AIController` (`AIBlueprintHelperLibrary.GetAIController` self)))
  (bind _blackboard (`AIController.Blackboard` _asbp_aicontroller))
  (`BlackboardComponent.SetValueAsBool` _blackboard "IsInteractedWith" true)
  (`BlackboardComponent.SetValueAsObject` _blackboard "PlayerActor" (`/Game/Base/BFL_BasicFunctions.GetPlayerCharacter`)))

(event `DialogueClosed`
  (bind _asbp_aicontroller (cast `/Game/NPC/AI/BP_AIController` (`AIBlueprintHelperLibrary.GetAIController` self)))
  (bind _blackboard (`AIController.Blackboard` _asbp_aicontroller))
  (`BlackboardComponent.SetValueAsBool` _blackboard "IsInteractedWith" false)
  (`BlackboardComponent.SetValueAsObject` _blackboard "PlayerActor" null))

(event `self.ReceiveActorBeginCursorOver`
  (`PrimitiveComponent.SetRenderCustomDepth` (`self.Mesh`) true))

(event `self.ReceiveActorEndCursorOver`
  (`PrimitiveComponent.SetRenderCustomDepth` (`self.Mesh`) false))

(fn `UserConstructionScript`)