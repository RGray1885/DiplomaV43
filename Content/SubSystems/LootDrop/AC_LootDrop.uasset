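; Actor component that drops loot around its owner, gated by the player's current level.
; DropLoot walks every loot data table row and, for each whose DropAtLevel is met, spawns one random class from that row.
; Spawns sit slightly above random reachable navmesh points near the owner.
; Each spawned mesh gets a small impulse, applied at a newly randomized location rather than its spawn point.
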(fn `DropLoot`
  (bind _randomlocation (`NavigationSystemV1.K2_GetRandomReachablePointInRadius` (.location (`Actor.GetTransform` (`self.GetOwner`))) 300.0 null null))
  (bind _returnvalue (`KismetMathLibrary.MakeVector` (.x _randomlocation) (.y _randomlocation) (+ (.z _randomlocation) 160.0)))
  (bind _outrownames (`DataTableFunctionLibrary.GetDataTableRowNames` (`self.LootDT`)))
  (for _array_element _outrownames
    (bind _returnvalue_2 (`|GetDataTableRow` (`self.LootDT`) _array_element)
      (:`then`
        (bind (_dropatlevel _lootclass) (break `/Game/SubSystems/LootDrop/S_LootDetails` _returnvalue_2))
        (if (>= (`/Game/SubSystems/PlayerStats/SystemFiles/AC_CharacterStats.CurrentLevel` (`/Game/Base/BFL_BasicFunctions.GetPlayerStatsSubsystem`)) _dropatlevel)
          (bind _returnvalue_3 (`|SpawnActorFromClass` (`KismetArrayLibrary.Array_Random` _lootclass) (`KismetMathLibrary.MakeTransform` _returnvalue) "Undefined" "OverrideRootScale" null null))
          (`/Engine/EditorBlueprintResources/StandardMacros.IsValid` _returnvalue_3
            (:`Is Valid`
              (`PrimitiveComponent.AddImpulseAtLocation` (`/Game/SubSystems/Inventory/Items/BP_ItemBase.StaticMesh` _returnvalue_3) (2.0 2.0 1.0) _returnvalue "None"))))))))