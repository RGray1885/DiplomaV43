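; AC_ItemInfoComponent is an inventory component that loads an item's definition from data tables at BeginPlay.
; Its data table row handle resolves to ItemInfo, whose nested handles optionally resolve to EquipmentInfo and AidInfo rows when their tables are valid.
; It then prints the item, aid and equipment class names as debug text, showing "None" for empty aid or equipment names.
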(event `self.ReceiveBeginPlay`
  (bind _aidinfo_aiditemclass (break `/Game/SubSystems/Inventory/SystemFiles/S_AidItemInfo` (`self.AidInfo`)))
  (bind _equipmentinfo_equipmentclass (break `/Game/SubSystems/Inventory/SystemFiles/S_EquipmentInfo` (`self.EquipmentInfo`)))
  (bind _returnvalue (`KismetSystemLibrary.GetClassDisplayName` _equipmentinfo_equipmentclass))
  (bind _returnvalue_2 (`KismetSystemLibrary.GetClassDisplayName` _aidinfo_aiditemclass))
  (`self.GetInfoFromDTH`)
  (`KismetSystemLibrary.PrintText` (`|FormatText` "Item {ItemClass} / Aid {AidClass} / Equip {EquipClass}" (`KismetSystemLibrary.GetClassDisplayName` (`.ItemClass_9_D0CE3054490C15AB80261FA45DC1E5FA` (break `/Game/SubSystems/Inventory/SystemFiles/S_ItemInfo` (`self.ItemInfo`)))) (select `bool` (`KismetStringLibrary.IsEmpty` _returnvalue_2) :`false` _returnvalue_2 :`true` " None") (select `bool` (`KismetStringLibrary.IsEmpty` _returnvalue) :`false` _returnvalue :`true` " None")) true true (struct :`G` 0.66 :`B` 1.0 :`A` 1.0) 10.0))

(fn `GetInfoFromDTH`
  (bind (_datatable _rowname) (break `DataTableRowHandle` (`self.ItemInfo_DTH`)))
  (bind _returnvalue (`|GetDataTableRow` _datatable _rowname)
    (:`then`
      (bind _output_get (set `self.ItemInfo` _returnvalue))
      (`|ExecutionSequence`
        (:`then_0`
          (bind (_itemclass _itemname _itemdescription _itemtype _itemcurrentamount _itemstacksize _itemprice _equipmentinfo _aiditeminfo) (break `/Game/SubSystems/Inventory/SystemFiles/S_ItemInfo` _output_get))
          (bind (_datatable_2 _rowname_2) (break `DataTableRowHandle` _equipmentinfo))
          (`/Engine/EditorBlueprintResources/StandardMacros.IsValid` _datatable_2
            (:`Is Valid`
              (bind _returnvalue_2 (`|GetDataTableRow` _datatable_2 _rowname_2)
                (:`then`
                  (set `self.EquipmentInfo` _returnvalue_2))))))
        (:`then_1`
          (bind (_datatable_3 _rowname_3) (break `DataTableRowHandle` _aiditeminfo))
          (`/Engine/EditorBlueprintResources/StandardMacros.IsValid` _datatable_3
            (:`Is Valid`
              (bind _returnvalue_3 (`|GetDataTableRow` _datatable_3 _rowname_3)
                (:`then`
                  (set `self.AidInfo` _returnvalue_3))))))))))