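; Equipment component that manages a character's equipment slots and reports stat bonuses and weapon pose state.
; It binds to the player inventory's pickup event, and its slot check spawns equipment for free slots using data table rows.
; EquipTo attaches hand weapons to mesh sockets, displacing conflicting items back into the inventory and destroying their actors.
; InitializeEquipment respawns the stored list; armor and accessory equipping are empty stubs.
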(event `self.ReceiveBeginPlay`
  (bind _ascharacter (cast `Character` (`self.GetOwner`)))
  (bind _output_get (set `self.ComponentOwner` _ascharacter))
  (bind _asbp_player (cast `/Game/Base/BP_Player` _output_get))
  (add `/Game/SubSystems/Inventory/SystemFiles/AC_Inventory.EquipmentPickedUp` (`/Game/Base/BP_Player.PlayerInventory` _asbp_player) (`|CreateDelegate` :!event `Check Equipment Slot`))
  (`KismetSystemLibrary.PrintString` "Event binded"))

(fn `Check Equipment Slot`
  (params (NewPickedItem :type "/Game/SubSystems/Inventory/SystemFiles/S_ItemInfo Structure"))
  (bind (_itemclass _itemname _itemdescription _itemtype _itemcurrentamount _itemstacksize _itemprice _equipmentinfo) (break `/Game/SubSystems/Inventory/SystemFiles/S_ItemInfo` NewPickedItem))
  (bind (_datatable _rowname) (break `DataTableRowHandle` _equipmentinfo))
  (bind _returnvalue (not (`KismetSystemLibrary.IsValid` (`self.TwoHandEquipment`))))
  (if (`|EnumEquality` _itemtype "NewEnumerator2")
    (bind _returnvalue_2 (`|GetDataTableRow` _datatable _rowname)
      (:`then`
        (bind (_equipmentclass _equipmenttype _equipmentslot) (break `/Game/SubSystems/Inventory/SystemFiles/S_EquipmentInfo` _returnvalue_2))
        (switch `/Game/SubSystems/Inventory/SystemFiles/E_EquipmentSlot` _equipmentslot
          (:`NewEnumerator0`
            (if (not (`KismetSystemLibrary.IsValid` (`self.ArmorEquipment`)))
              (bind _returnvalue_3 (`|SpawnActorFromClass` _equipmentclass (`Actor.GetTransform` (`self.GetOwner`)) "Undefined" "OverrideRootScale" null NewPickedItem null :!label _label))
              (`self.EquipTo` _returnvalue_3)))
          (:`NewEnumerator1`
            (if (not (`KismetSystemLibrary.IsValid` (`self.MainHandEquipment`)))
              (if _returnvalue
                (goto _label))))
          (:`NewEnumerator2`
            (if (not (`KismetSystemLibrary.IsValid` (`self.OffHandEquipment`)))
              (if _returnvalue
                (goto _label))))
          (:`NewEnumerator3`
            (if (not (`KismetSystemLibrary.IsValid` (`self.AccessoryEquipment`)))
              (goto _label)))
          (:`NewEnumerator4`
            (if _returnvalue
              (goto _label))))))))

(fn `EquipAccessory`
  (params (Equipment :type "/Game/SubSystems/Inventory/Equipment/BP_EquipmentBasic Object Reference")))

(fn `EquipArmor`
  (params (Equipment :type "/Game/SubSystems/Inventory/Equipment/BP_EquipmentBasic Object Reference")))

(fn `EquipTo`
  (params (ItemToEquip :type "/Game/SubSystems/Inventory/Equipment/BP_EquipmentBasic Object Reference"))
  (bind _itemtoequip (`local.ItemToEquip`))
  (bind (_itemclass _itemname _itemdescription _itemtype _itemcurrentamount _itemstacksize _itemprice _equipmentinfo) (break `/Game/SubSystems/Inventory/SystemFiles/S_ItemInfo` (`/Game/SubSystems/Inventory/Equipment/BP_EquipmentBasic.ItemInfo` ItemToEquip)))
  (bind (_datatable _rowname) (break `DataTableRowHandle` _equipmentinfo))
  (if (`|EnumEquality` _itemtype "NewEnumerator2")
    (bind _returnvalue (`|GetDataTableRow` _datatable _rowname)
      (:`then`
        (switch `/Game/SubSystems/Inventory/SystemFiles/E_EquipmentSlot` (`.EquipmentSlot_25_A9E74878467C51A95BFF90B42A72CCB3` (break `/Game/SubSystems/Inventory/SystemFiles/S_EquipmentInfo` _returnvalue))
          (:`NewEnumerator0`
            (`self.EquipArmor` _itemtoequip))
          (:`NewEnumerator1`
            (`self.EquipToMainHand` _itemtoequip))
          (:`NewEnumerator2`
            (`self.EquipToOffHand` _itemtoequip))
          (:`NewEnumerator3`
            (`self.EquipAccessory` _itemtoequip))
          (:`NewEnumerator4`
            (`self.EquipToTwoHandSlot` _itemtoequip)))
        (`self.EquipmentChanged`)))))

(fn `EquipToMainHand`
  (params (Equipment :type "/Game/SubSystems/Inventory/Equipment/BP_EquipmentBasic Object Reference"))
  (bind _twohandequipment (`self.TwoHandEquipment`))
  (bind (_itemclass _itemname _itemdescription _itemtype _itemcurrentamount _itemstacksize _itemprice _equipmentinfo _aiditeminfo _icon _iteminventoryindex) (break `/Game/SubSystems/Inventory/SystemFiles/S_ItemInfo` (`/Game/SubSystems/Inventory/Equipment/BP_EquipmentBasic.ItemInfo` Equipment)))
  (bind _s_iteminfo (make `/Game/SubSystems/Inventory/SystemFiles/S_ItemInfo` _itemclass _itemname _itemdescription _itemtype 1 _itemstacksize _itemprice _equipmentinfo _aiditeminfo _icon _iteminventoryindex))
  (`/Engine/EditorBlueprintResources/StandardMacros.IsValid` _twohandequipment
    (:`Is Valid`
      (`self.RemoveEquipment` _twohandequipment :!label _label))
    (:`Is Not Valid`
      (`/Engine/EditorBlueprintResources/StandardMacros.IsValid` (`self.MainHandEquipment`)
        (:`Is Valid`
          (goto _label))
        (:`Is Not Valid`
          _))))
  (`Actor.K2_AttachToComponent` Equipment (`Character.Mesh` (`self.ComponentOwner`)) "RightHandSocket" "SnapToTarget" "SnapToTarget" "SnapToTarget" true)
  (`KismetArrayLibrary.Array_Add` (`self.Equipment`) _s_iteminfo)
  (set `self.MainHandEquipment` Equipment)
  (`/Game/SubSystems/Inventory/SystemFiles/AC_Inventory.RemoveFromInventory` (`/Game/Base/BP_Player.PlayerInventory` (`/Game/Base/BFL_BasicFunctions.GetPlayerCharacter`)) _s_iteminfo))

(fn `EquipToOffHand`
  (params (Equipment :type "/Game/SubSystems/Inventory/Equipment/BP_EquipmentBasic Object Reference"))
  (bind _twohandequipment (`self.TwoHandEquipment`))
  (bind _offhandequipment (`self.OffHandEquipment`))
  (bind (_itemclass _itemname _itemdescription _itemtype _itemcurrentamount _itemstacksize _itemprice _equipmentinfo _aiditeminfo _icon _iteminventoryindex) (break `/Game/SubSystems/Inventory/SystemFiles/S_ItemInfo` (`/Game/SubSystems/Inventory/Equipment/BP_EquipmentBasic.ItemInfo` Equipment)))
  (bind _s_iteminfo (make `/Game/SubSystems/Inventory/SystemFiles/S_ItemInfo` _itemclass _itemname _itemdescription _itemtype 1 _itemstacksize _itemprice _equipmentinfo _aiditeminfo _icon _iteminventoryindex))
  (`/Engine/EditorBlueprintResources/StandardMacros.IsValid` _twohandequipment
    (:`Is Valid`
      (`self.RemoveEquipment` _twohandequipment))
    (:`Is Not Valid`
      (`/Engine/EditorBlueprintResources/StandardMacros.IsValid` _offhandequipment
        (:`Is Valid`
          (`self.RemoveEquipment` _offhandequipment))
        (:`Is Not Valid`
          _))))
  (`Actor.K2_AttachToComponent` Equipment (`Character.Mesh` (`self.ComponentOwner`)) "LeftHandSocket" "SnapToTarget" "SnapToTarget" "SnapToTarget" true)
  (`KismetArrayLibrary.Array_Add` (`self.Equipment`) _s_iteminfo)
  (set `self.OffHandEquipment` Equipment)
  (`/Game/SubSystems/Inventory/SystemFiles/AC_Inventory.RemoveFromInventory` (`/Game/Base/BP_Player.PlayerInventory` (`/Game/Base/BFL_BasicFunctions.GetPlayerCharacter`)) _s_iteminfo))

(fn `EquipToTwoHandSlot`
  (params (Equipment :type "/Game/SubSystems/Inventory/Equipment/BP_EquipmentBasic Object Reference"))
  (bind _mainhandequipment (`self.MainHandEquipment`))
  (bind _offhandequipment (`self.OffHandEquipment`))
  (bind (_itemclass _itemname _itemdescription _itemtype _itemcurrentamount _itemstacksize _itemprice _equipmentinfo _aiditeminfo _icon _iteminventoryindex) (break `/Game/SubSystems/Inventory/SystemFiles/S_ItemInfo` (`/Game/SubSystems/Inventory/Equipment/BP_EquipmentBasic.ItemInfo` Equipment)))
  (bind _s_iteminfo (make `/Game/SubSystems/Inventory/SystemFiles/S_ItemInfo` _itemclass _itemname _itemdescription _itemtype 1 _itemstacksize _itemprice _equipmentinfo _aiditeminfo _icon _iteminventoryindex))
  (`/Engine/EditorBlueprintResources/StandardMacros.IsValid` _mainhandequipment
    (:`Is Valid`
      (`self.RemoveEquipment` _mainhandequipment))
    (:`Is Not Valid`
      _))
  (`/Engine/EditorBlueprintResources/StandardMacros.IsValid` _offhandequipment
    (:`Is Valid`
      (`self.RemoveEquipment` _offhandequipment))
    (:`Is Not Valid`
      _))
  (`Actor.K2_AttachToComponent` Equipment (`Character.Mesh` (`self.ComponentOwner`)) "RightHandSocket" "SnapToTarget" "SnapToTarget" "SnapToTarget" true)
  (`KismetArrayLibrary.Array_Add` (`self.Equipment`) _s_iteminfo)
  (set `self.TwoHandEquipment` Equipment)
  (`/Game/SubSystems/Inventory/SystemFiles/AC_Inventory.RemoveFromInventory` (`/Game/Base/BP_Player.PlayerInventory` (`/Game/Base/BFL_BasicFunctions.GetPlayerCharacter`)) _s_iteminfo))

(fn `GetEquipmentState`
  (returns (SwordAndShield :type Boolean) (TwoHanded :type Boolean) (PoseOneHand :type Boolean) (PoseUnarmed :type Boolean))
  (bind _returnvalue (`KismetSystemLibrary.IsValid` (`self.MainHandEquipment`)))
  (bind _returnvalue_2 (`KismetSystemLibrary.IsValid` (`self.OffHandEquipment`)))
  (if (`KismetSystemLibrary.IsValid` (`self.TwoHandEquipment`))
    (set `self.PoseTwoHanded` true)
    (set `self.PoseSwordAndShield` false)
    (set `self.PoseOneHand` false)
    (set `self.PoseUnarmed` false)
    (elif (and _returnvalue _returnvalue_2)
      (set `self.PoseSwordAndShield` true)
      (set `self.PoseTwoHanded` false)
      (set `self.PoseOneHand` false)
      (set `self.PoseUnarmed` false)
      (elif (or _returnvalue _returnvalue_2)
        (set `self.PoseOneHand` true)
        (set `self.PoseUnarmed` false)
        (set `self.PoseTwoHanded` false)
        (set `self.PoseSwordAndShield` false)
        (else
          (set `self.PoseUnarmed` true)
          (set `self.PoseSwordAndShield` false)
          (set `self.PoseTwoHanded` false)
          (set `self.PoseOneHand` false)))))
  (return (`self.PoseSwordAndShield`) (`self.PoseTwoHanded`) (`self.PoseOneHand`) (`self.PoseUnarmed`)))

(fn `GetRequiredEquipment`
  (params (EquipmentSlot :type "/Game/SubSystems/Inventory/SystemFiles/E_EquipmentSlot Enum" :default "NewEnumerator0"))
  (returns (RequiredEquipment :type "/Game/SubSystems/Inventory/Equipment/BP_EquipmentBasic Object Reference"))
  (return (select `/Game/SubSystems/Inventory/SystemFiles/E_EquipmentSlot` EquipmentSlot :`NewEnumerator0` (`self.ArmorEquipment`) :`NewEnumerator1` (`self.MainHandEquipment`) :`NewEnumerator2` (`self.OffHandEquipment`) :`NewEnumerator3` (`self.AccessoryEquipment`) :`NewEnumerator4` (`self.TwoHandEquipment`))))

(fn `GetSummarizedStats`
  (returns (EquipDamageBonusMin :type Integer) (EquipDamageBonusMax :type Integer) (EquipDefenseBonusMin :type Integer) (EquipDefenseBonusMax :type Integer))
  (locals (EquipDamageMin :type Integer) (EquipDamageMax :type Integer) (EquipDefenseMin :type Integer) (EquipDefenseMax :type Integer))
  (for _array_element (`self.Equipment`)
    (bind (_datatable _rowname) (break `DataTableRowHandle` (`.EquipmentInfo_38_F72D43004768FCF4953CF38D6FA6EDE3` (break `/Game/SubSystems/Inventory/SystemFiles/S_ItemInfo` _array_element))))
    (bind _returnvalue (`|GetDataTableRow` _datatable _rowname)
      (:`then`
        (bind ((`DamageBonus_32_EFF5A90349C39449E5CAB19B412A4C5D` _damagebonus) (`DefenseBonus_31_C35348C4430564B85C86978DE1900624` _defensebonus)) (break `/Game/SubSystems/Inventory/SystemFiles/S_EquipmentInfo` _returnvalue))
        (set `local.EquipDamageMin` (+ (`local.EquipDamageMin`) _damagebonus))
        (set `local.EquipDamageMax` (+ (`local.EquipDamageMax`) _damagebonus))
        (set `local.EquipDefenseMin` (+ (`local.EquipDefenseMin`) 1))
        (set `local.EquipDefenseMax` (+ (`local.EquipDefenseMax`) _defensebonus)))))
  (return (`local.EquipDamageMin`) (`local.EquipDamageMax`) (`local.EquipDefenseMin`) (`local.EquipDefenseMax`)))

(fn `InitializeEquipment`
  (locals (WeaponFound :type Boolean))
  (bind _equipment (`self.Equipment`))
  (if (> (`KismetArrayLibrary.Array_Length` _equipment) 0)
    (for _array_element _equipment
      (if (== (`.ItemClass_9_D0CE3054490C15AB80261FA45DC1E5FA` (break `/Game/SubSystems/Inventory/SystemFiles/S_ItemInfo` _array_element)) "/Game/SubSystems/Inventory/Items/Weapons/BP_ItemBaseWeapon.BP_ItemBaseWeapon_C")
        (set `local.WeaponFound` true))
      (bind ((`EquipmentInfo_38_F72D43004768FCF4953CF38D6FA6EDE3` _equipmentinfo)) (break `/Game/SubSystems/Inventory/SystemFiles/S_ItemInfo` _array_element))
      (bind _returnvalue (`|GetDataTableRow` (break `DataTableRowHandle` _equipmentinfo) (`.RowName` (break `DataTableRowHandle` _equipmentinfo)))
        (:`then`
          (bind _returnvalue_2 (`|SpawnActorFromClass` (`.EquipmentClass_2_4DD88FF2403FBF68A1ACF88CD044EF53` (break `/Game/SubSystems/Inventory/SystemFiles/S_EquipmentInfo` _returnvalue)) (`Actor.GetTransform` (`self.GetOwner`)) "Undefined" "OverrideRootScale" null _array_element null))
          (`self.EquipTo` _returnvalue_2))))))

(fn `RemoveEquipment`
  (params (EquipmentToRemove :type "/Game/SubSystems/Inventory/Equipment/BP_EquipmentBasic Object Reference"))
  (bind _iteminfo (`/Game/SubSystems/Inventory/Equipment/BP_EquipmentBasic.ItemInfo` EquipmentToRemove))
  (bind _equipment (`self.Equipment`))
  (`/Engine/EditorBlueprintResources/StandardMacros.IsValid` EquipmentToRemove
    (:`Is Valid`
      (if (not (not (== EquipmentToRemove (`self.TwoHandEquipment`))))
        (bind _aswbp_inventory_ui (cast `/Game/SubSystems/Inventory/UI/WBP_Inventory_UI` (`PanelWidget.GetChildAt` (`/Game/Base/WBP_Player_UI.InventoryCanvas` (`/Game/Base/BP_Player_HUD.PlayerUI_Ref` (`/Game/Base/BFL_BasicFunctions.Get Player HUD`))) 0)))
        (set `/Game/SubSystems/Inventory/UI/WBP_EquipmentIcon.ItemInfo` (struct) (`/Game/SubSystems/Inventory/UI/WBP_Inventory_UI.WBP_EquipmentIcon_MainHand` _aswbp_inventory_ui))
        (set `/Game/SubSystems/Inventory/UI/WBP_EquipmentIcon.ItemInfo` (struct) (`/Game/SubSystems/Inventory/UI/WBP_Inventory_UI.WBP_EquipmentIcon_OffHand` _aswbp_inventory_ui)))
      (bind _returnvalue (`KismetArrayLibrary.Array_RemoveItem` _equipment _iteminfo))
      (if _returnvalue
        (`/Game/SubSystems/Inventory/SystemFiles/AC_Inventory.AddToInventory` (`/Game/Base/BP_Player.PlayerInventory` (`/Game/Base/BFL_BasicFunctions.GetPlayerCharacter`)) _iteminfo :!label _label)
        (`Actor.K2_DetachFromActor` EquipmentToRemove "KeepRelative" "KeepRelative" "KeepRelative")
        (`KismetSystemLibrary.PrintString` (`KismetStringLibrary.Concat_StrStr` (`KismetSystemLibrary.GetDisplayName` EquipmentToRemove) " removed"))
        (`Actor.K2_DestroyActor` EquipmentToRemove)
        (`self.EquipmentChanged`)
        (else
          (for _array_element _equipment
            (if (== (`.ItemClass_9_D0CE3054490C15AB80261FA45DC1E5FA` (break `/Game/SubSystems/Inventory/SystemFiles/S_ItemInfo` _array_element)) (`.ItemClass_9_D0CE3054490C15AB80261FA45DC1E5FA` (break `/Game/SubSystems/Inventory/SystemFiles/S_ItemInfo` _iteminfo)))
              (`KismetArrayLibrary.Array_RemoveItem` _equipment _array_element)
              (goto _label))))))))

(fn `SetBasicEquipment`
  (params (EquipmentType :type Name))
  (switch `name` EquipmentType))