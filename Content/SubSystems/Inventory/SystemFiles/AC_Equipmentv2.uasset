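; Character equipment component that manages armor, accessory, main-hand, off-hand and ranged gear, granting a starter bow, sword and shield on BeginPlay.
; Equipping spawns the actor class from the item's data table row, attaches it by slot and swaps items with BP_Player's inventory.
; Sheathing, melee/ranged switching and two-hand toggling move gear between back and hand sockets.
; GetStance derives the stance from in-hand items and toggles the owner's controller-yaw rotation.
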(event `self.ReceiveBeginPlay`
  (`self.Set Starter Equipment` "Ranged")
  (`self.Set Starter Equipment` "SwordAndShield"))

(fn `EquipItem`
  (params (ItemInfo :type "/Game/SubSystems/Inventory/SystemFiles/S_ItemInfo Structure"))
  (locals (SocketToAttach :type Name) (Owner :type "Character Object Reference") (ItemEquippedInfo :type "/Game/SubSystems/Inventory/SystemFiles/S_ItemInfo Structure") (EquippedItemActor :type "/Game/SubSystems/Inventory/Equipment/BP_EquipmentBasic Object Reference"))
  (bind _itemequippedinfo (`local.ItemEquippedInfo`))
  (bind _equipmentoncharacter (`self.EquipmentOnCharacter`))
  (bind _owner (`local.Owner`))
  (bind (_datatable _rowname) (break `DataTableRowHandle` (`.EquipmentInfo_38_F72D43004768FCF4953CF38D6FA6EDE3` (break `/Game/SubSystems/Inventory/SystemFiles/S_ItemInfo` ItemInfo))))
  (bind (_asbp_player _bsuccess) (cast `/Game/Base/BP_Player` (`local.Owner`) :!pure true))
  (bind _playerinventory (`/Game/Base/BP_Player.PlayerInventory` _asbp_player))
  (bind _ascharacter (cast `Character` (`self.GetOwner`)))
  (set `local.Owner` _ascharacter)
  (bind _returnvalue (`|GetDataTableRow` _datatable _rowname)
    (:`then`
      (bind (_equipmentclass _equipmenttype _equipmentslot) (break `/Game/SubSystems/Inventory/SystemFiles/S_EquipmentInfo` _returnvalue))
      (bind _returnvalue_2 (`|SpawnActorFromClass` _equipmentclass (`Actor.GetTransform` _owner) "Undefined" "OverrideRootScale" null ItemInfo null))
      (switch `/Game/SubSystems/Inventory/SystemFiles/E_EquipmentSlot` _equipmentslot
        (:`NewEnumerator0`
          (set `local.SocketToAttach` "None")
          (bind _armorequipment (`self.ArmorEquipment`)
            (:`then`
              (set `local.ItemEquippedInfo` (`/Game/SubSystems/Inventory/Equipment/BP_EquipmentBasic.ItemInfo` _armorequipment))
              (set `local.EquippedItemActor` _armorequipment)
              (`|ExecutionSequence`
                (:`then_0`
                  (if _bsuccess :!label _label
                    (`/Game/SubSystems/Inventory/SystemFiles/AC_Inventory.AddToInventory` _playerinventory _itemequippedinfo))
                  (`Actor.K2_DetachFromActor` (`local.EquippedItemActor`) "KeepRelative" "KeepRelative" "KeepRelative"))
                (:`then_1`
                  (set `self.ArmorEquipment` _returnvalue_2 :!label _label_2))))
            (:`else`
              (goto _label_2))))
        (:`NewEnumerator1`
          (`self.MeleeWeaponInHand`
            (:`then`
              (set `local.SocketToAttach` "RightHandSocket"))
            (:`else`
              (set `local.SocketToAttach` "EquipmentOnBack_MainHand")))
          (bind _mainhandequipment (`self.MainHandEquipment`)
            (:`then`
              (set `local.ItemEquippedInfo` (`/Game/SubSystems/Inventory/Equipment/BP_EquipmentBasic.ItemInfo` _mainhandequipment))
              (set `local.EquippedItemActor` _mainhandequipment)
              (`|ExecutionSequence`
                (:`then_0`
                  (goto _label))
                (:`then_1`
                  _)))
            (:`else`
              _))
          (set `self.MainHandEquipment` _returnvalue_2))
        (:`NewEnumerator2`
          (`self.ShieldInHand`
            (:`then`
              (set `local.SocketToAttach` "LeftHandSocket"))
            (:`else`
              (set `local.SocketToAttach` "EquipmentOnBack_Shield")))
          (bind _offhandequipment (`self.OffHandEquipment`)
            (:`then`
              (set `local.ItemEquippedInfo` (`/Game/SubSystems/Inventory/Equipment/BP_EquipmentBasic.ItemInfo` _offhandequipment))
              (set `local.EquippedItemActor` _offhandequipment)
              (`|ExecutionSequence`
                (:`then_0`
                  (goto _label))
                (:`then_1`
                  _)))
            (:`else`
              _))
          (set `self.OffHandEquipment` _returnvalue_2))
        (:`NewEnumerator3`
          (set `local.SocketToAttach` "None")
          (bind _accessoryequipment (`self.AccessoryEquipment`)
            (:`then`
              (set `local.ItemEquippedInfo` (`/Game/SubSystems/Inventory/Equipment/BP_EquipmentBasic.ItemInfo` _accessoryequipment))
              (set `local.EquippedItemActor` _accessoryequipment)
              (`|ExecutionSequence`
                (:`then_0`
                  (goto _label))
                (:`then_1`
                  _)))
            (:`else`
              _))
          (set `self.AccessoryEquipment` _returnvalue_2))
        (:`NewEnumerator4`
          (`self.RangedInHand`
            (:`then`
              (set `local.SocketToAttach` "LeftHandRangedSocket"))
            (:`else`
              (set `local.SocketToAttach` "EquipmentOnBack_Ranged")))
          (bind _rangedequipment (`self.RangedEquipment`)
            (:`then`
              (set `local.ItemEquippedInfo` (`/Game/SubSystems/Inventory/Equipment/BP_EquipmentBasic.ItemInfo` _rangedequipment))
              (set `local.EquippedItemActor` _rangedequipment)
              (`|ExecutionSequence`
                (:`then_0`
                  (goto _label))
                (:`then_1`
                  _)))
            (:`else`
              _))
          (set `self.RangedEquipment` _returnvalue_2)))
      (`Actor.K2_AttachToComponent` _returnvalue_2 (`Character.Mesh` _owner) (`local.SocketToAttach`) "SnapToTarget" "SnapToTarget" "SnapToTarget" true)
      (`/Game/SubSystems/Inventory/SystemFiles/AC_Inventory.RemoveFromInventory` _playerinventory ItemInfo)
      (`KismetArrayLibrary.Array_RemoveItem` _equipmentoncharacter _itemequippedinfo)
      (`KismetArrayLibrary.Array_Add` _equipmentoncharacter ItemInfo))
    (:`RowNotFound`
      (`KismetSystemLibrary.PrintString` "Not an Equipment"))))

(fn `GetStance`
  (bind _returnvalue (`KismetSystemLibrary.IsValid` (`self.MeleeWeaponInHand`)))
  (bind _returnvalue_2 (`KismetSystemLibrary.IsValid` (`self.ShieldInHand`)))
  (if (and _returnvalue _returnvalue_2)
    (`KismetSystemLibrary.PrintString` "SwordAndShield")
    (set `self.CurrentStance` "NewEnumerator4")
    (bind _ascharacter (cast `Character` (`self.GetOwner`) :!label _label))
    (set `Pawn.bUseControllerRotationYaw` true _ascharacter)
    (elif (and _returnvalue (not _returnvalue_2))
      (`KismetSystemLibrary.PrintString` "Singlehand")
      (set `self.CurrentStance` "NewEnumerator1")
      (goto _label)
      (elif (`KismetSystemLibrary.IsValid` (`self.RangedInHand`))
        (`KismetSystemLibrary.PrintString` "Ranged")
        (set `self.CurrentStance` "NewEnumerator2")
        (goto _label)
        (else
          (`KismetSystemLibrary.PrintString` "Unarmed")
          (set `self.CurrentStance` "NewEnumerator3")
          (bind _ascharacter_2 (cast `Character` (`self.GetOwner`)))
          (set `Pawn.bUseControllerRotationYaw` false _ascharacter_2))))))

(fn `GetWeaponInHand`
  (returns (WeaponInHand1 :type "/Game/SubSystems/Inventory/Equipment/BP_EquipmentBasic Object Reference"))
  (locals (WeaponInHand :type "/Game/SubSystems/Inventory/Equipment/BP_EquipmentBasic Object Reference"))
  (bind _meleeweaponinhand (`self.MeleeWeaponInHand`)
    (:`then`
      (set `local.WeaponInHand` _meleeweaponinhand))
    (:`else`
      (bind _rangedinhand (`self.RangedInHand`)
        (:`then`
          (set `local.WeaponInHand` _rangedinhand))
        (:`else`
          (set `local.WeaponInHand` null)))))
  (return (`local.WeaponInHand`)))

(fn `Set Starter Equipment`
  (params (StarterSet :type Name))
  (bind _returnvalue (`self.GetOwner`))
  (bind _equipmentoncharacter (`self.EquipmentOnCharacter`))
  (bind _returnvalue_2 (`Actor.GetTransform` _returnvalue))
  (bind _ascharacter (cast `Character` _returnvalue))
  (switch `name` StarterSet
    (:`SwordAndShield`
      (`|ExecutionSequence`
        (:`then_0`
          (bind _returnvalue_3 (`|SpawnActorFromClass` "/Game/SubSystems/Inventory/Items/Shields/BP_Item_OldShield.BP_Item_OldShield_C" _returnvalue_2 "Undefined" "OverrideRootScale" null null))
          (bind _iteminfo (`/Game/SubSystems/Inventory/SystemFiles/AC_ItemInfoComponent.ItemInfo` (`/Game/SubSystems/Inventory/Items/BP_ItemBase.ItemInfoComponent` _returnvalue_3)))
          (bind (_datatable _rowname) (break `DataTableRowHandle` (`.EquipmentInfo_38_F72D43004768FCF4953CF38D6FA6EDE3` (break `/Game/SubSystems/Inventory/SystemFiles/S_ItemInfo` _iteminfo))))
          (bind _returnvalue_4 (`|GetDataTableRow` _datatable _rowname)
            (:`then`
              (bind (_equipmentclass _equipmenttype _equipmentslot) (break `/Game/SubSystems/Inventory/SystemFiles/S_EquipmentInfo` _returnvalue_4))
              (bind _returnvalue_5 (`|SpawnActorFromClass` _equipmentclass _returnvalue_2 "Undefined" "OverrideRootScale" null _iteminfo null))
              (switch `/Game/SubSystems/Inventory/SystemFiles/E_EquipmentSlot` _equipmentslot
                (:`NewEnumerator1`
                  (bind _mesh (`Character.Mesh` _ascharacter))
                  (`Actor.K2_AttachToComponent` _returnvalue_5 _mesh "EquipmentOnBack_MainHand" "SnapToTarget" "SnapToTarget" "SnapToTarget" true)
                  (bind _output_get (set `self.MainHandEquipment` _returnvalue_5))
                  (`KismetArrayLibrary.Array_AddUnique` _equipmentoncharacter (`/Game/SubSystems/Inventory/Equipment/BP_EquipmentBasic.ItemInfo` _output_get)))
                (:`NewEnumerator2`
                  (`Actor.K2_AttachToComponent` _returnvalue_5 _mesh "EquipmentOnBack_Shield" "SnapToTarget" "SnapToTarget" "SnapToTarget" true)
                  (bind _output_get_2 (set `self.OffHandEquipment` _returnvalue_5))
                  (`KismetArrayLibrary.Array_AddUnique` _equipmentoncharacter (`/Game/SubSystems/Inventory/Equipment/BP_EquipmentBasic.ItemInfo` _output_get_2))))
              (`Actor.K2_DestroyActor` _returnvalue_3))))
        (:`then_1`
          (bind _returnvalue_6 (`|SpawnActorFromClass` "/Game/SubSystems/Inventory/Items/Weapons/BP_ItemRustedSword.BP_ItemRustedSword_C" _returnvalue_2 "Undefined" "OverrideRootScale" null null :!label _label))
          (bind _iteminfo_2 (`/Game/SubSystems/Inventory/SystemFiles/AC_ItemInfoComponent.ItemInfo` (`/Game/SubSystems/Inventory/Items/BP_ItemBase.ItemInfoComponent` _returnvalue_6)))
          (bind (_datatable_2 _rowname_2) (break `DataTableRowHandle` (`.EquipmentInfo_38_F72D43004768FCF4953CF38D6FA6EDE3` (break `/Game/SubSystems/Inventory/SystemFiles/S_ItemInfo` _iteminfo_2))))
          (bind _returnvalue_7 (`|GetDataTableRow` _datatable_2 _rowname_2)
            (:`then`
              (bind ((`EquipmentClass_2_4DD88FF2403FBF68A1ACF88CD044EF53` _equipmentclass_2) (`EquipmentSlot_25_A9E74878467C51A95BFF90B42A72CCB3` _equipmentslot_2)) (break `/Game/SubSystems/Inventory/SystemFiles/S_EquipmentInfo` _returnvalue_7))
              (bind _returnvalue_8 (`|SpawnActorFromClass` _equipmentclass_2 _returnvalue_2 "Undefined" "OverrideRootScale" null _iteminfo_2 null))
              (switch `/Game/SubSystems/Inventory/SystemFiles/E_EquipmentSlot` _equipmentslot_2
                (:`NewEnumerator1`
                  (`Actor.K2_AttachToComponent` _returnvalue_8 _mesh "EquipmentOnBack_MainHand" "SnapToTarget" "SnapToTarget" "SnapToTarget" true)
                  (bind _output_get_3 (set `self.MainHandEquipment` _returnvalue_8))
                  (`KismetArrayLibrary.Array_AddUnique` _equipmentoncharacter (`/Game/SubSystems/Inventory/Equipment/BP_EquipmentBasic.ItemInfo` _output_get_3)))
                (:`NewEnumerator2`
                  (`Actor.K2_AttachToComponent` _returnvalue_8 _mesh "EquipmentOnBack_Shield" "SnapToTarget" "SnapToTarget" "SnapToTarget" true)
                  (bind _output_get_4 (set `self.OffHandEquipment` _returnvalue_8))
                  (`KismetArrayLibrary.Array_AddUnique` _equipmentoncharacter (`/Game/SubSystems/Inventory/Equipment/BP_EquipmentBasic.ItemInfo` _output_get_4))))
              (`Actor.K2_DestroyActor` _returnvalue_6))))))
    (:`Ranged`
      (bind _returnvalue_9 (`|SpawnActorFromClass` "/Game/SubSystems/Inventory/Items/Weapons/BP_ItemBow.BP_ItemBow_C" _returnvalue_2 "Undefined" "OverrideRootScale" null null))
      (bind _iteminfo_3 (`/Game/SubSystems/Inventory/SystemFiles/AC_ItemInfoComponent.ItemInfo` (`/Game/SubSystems/Inventory/Items/BP_ItemBase.ItemInfoComponent` _returnvalue_9)))
      (bind (_datatable_3 _rowname_3) (break `DataTableRowHandle` (`.EquipmentInfo_38_F72D43004768FCF4953CF38D6FA6EDE3` (break `/Game/SubSystems/Inventory/SystemFiles/S_ItemInfo` _iteminfo_3))))
      (bind _returnvalue_10 (`|GetDataTableRow` _datatable_3 _rowname_3)
        (:`then`
          (bind (_equipmentclass_3 _equipmenttype_2 _equipmentslot_3) (break `/Game/SubSystems/Inventory/SystemFiles/S_EquipmentInfo` _returnvalue_10))
          (bind _returnvalue_11 (`|SpawnActorFromClass` _equipmentclass_3 _returnvalue_2 "Undefined" "OverrideRootScale" null _iteminfo_3 null))
          (switch `/Game/SubSystems/Inventory/SystemFiles/E_EquipmentSlot` _equipmentslot_3
            (:`NewEnumerator4`
              (`Actor.K2_AttachToComponent` _returnvalue_11 _mesh "EquipmentOnBack_Ranged" "SnapToTarget" "SnapToTarget" "SnapToTarget" true)
              (bind _output_get_5 (set `self.RangedEquipment` _returnvalue_11))
              (`KismetArrayLibrary.Array_AddUnique` _equipmentoncharacter (`/Game/SubSystems/Inventory/Equipment/BP_EquipmentBasic.ItemInfo` _output_get_5))
              (`Actor.K2_DestroyActor` _returnvalue_9))))))
    (:`OneHanded`
      (goto _label)))
  (`self.GetStance`))

(fn `SwitchMeleeRangedWeapon`
  (bind _ascharacter (cast `Character` (`self.GetOwner`)))
  (if (`self.CurrentWeaponIsMelee?`)
    (bind _rangedequipment (`self.RangedEquipment`)
      (:`then`
        (bind _offhandequipment (`self.OffHandEquipment`)
          (:`then`
            (bind _mesh (`Character.Mesh` _ascharacter))
            (`Actor.K2_AttachToComponent` _offhandequipment _mesh "EquipmentOnBack_Shield" "SnapToTarget" "SnapToTarget" "SnapToTarget" true))
          (:`else`
            _))
        (bind _mainhandequipment (`self.MainHandEquipment`)
          (:`then`
            (`Actor.K2_AttachToComponent` _mainhandequipment _mesh "EquipmentOnBack_MainHand" "SnapToTarget" "SnapToTarget" "SnapToTarget" true))
          (:`else`
            _))
        (set `self.CurrentWeaponIsMelee?` false)
        (`Actor.K2_AttachToComponent` _rangedequipment _mesh "LeftHandRangedSocket" "SnapToTarget" "SnapToTarget" "SnapToTarget" true)
        (set `self.RangedInHand` _rangedequipment)
        (set `self.ShieldInHand` null)
        (set `self.MeleeWeaponInHand` null))
      (:`else`))
    (else
      (bind _mainhandequipment_2 (`self.MainHandEquipment`)
        (:`then`
          (bind _rangedequipment_2 (`self.RangedEquipment`)
            (:`then`
              (`Actor.K2_AttachToComponent` _rangedequipment_2 _mesh "EquipmentOnBack_Ranged" "SnapToTarget" "SnapToTarget" "SnapToTarget" true)
              (bind _offhandequipment_2 (`self.OffHandEquipment`)
                (:`then`
                  (`Actor.K2_AttachToComponent` _offhandequipment_2 _mesh "LeftHandSocket" "SnapToTarget" "SnapToTarget" "SnapToTarget" true))
                (:`else`
                  _))
              (`Actor.K2_AttachToComponent` _mainhandequipment_2 _mesh "RightHandSocket" "SnapToTarget" "SnapToTarget" "SnapToTarget" true)
              (set `self.CurrentWeaponIsMelee?` true)
              (set `self.RangedInHand` null)
              (set `self.ShieldInHand` _offhandequipment_2)
              (set `self.MeleeWeaponInHand` _mainhandequipment_2))
            (:`else`)))
        (:`else`))))
  (`self.GetStance`))

(fn `SwitchToTwoHandStance`
  (bind _weaponinhand1 (`self.GetWeaponInHand`))
  (`/Engine/EditorBlueprintResources/StandardMacros.IsValid` _weaponinhand1
    (:`Is Valid`
      (if (`|EnumInequality` (`self.CurrentStance`) "NewEnumerator2")
        (if (`|EnumInequality` (`self.CurrentStance`) "NewEnumerator0")
          (bind _offhandequipment (`self.OffHandEquipment`)
            (:`then`
              (bind _ascharacter (cast `Character` (`self.GetOwner`)))
              (`Actor.K2_AttachToComponent` _offhandequipment (`Character.Mesh` _ascharacter) "EquipmentOnBack_Shield" "SnapToTarget" "SnapToTarget" "SnapToTarget" true))
            (:`else`
              _))
          (set `self.CurrentStance` "NewEnumerator0")
          (else
            (bind _offhandequipment_2 (`self.OffHandEquipment`)
              (:`then`
                (bind _ascharacter_2 (cast `Character` (`self.GetOwner`)))
                (`Actor.K2_AttachToComponent` _offhandequipment_2 (`Character.Mesh` _ascharacter_2) "LeftHandSocket" "SnapToTarget" "SnapToTarget" "SnapToTarget" true)
                (set `self.CurrentStance` "NewEnumerator4"))
              (:`else`
                (set `self.CurrentStance` "NewEnumerator1")))))))))

(fn `Toggle Sheath Weapon`
  (bind _rangedequipment (`self.RangedEquipment`))
  (bind _ascharacter (cast `Character` (`self.GetOwner`)))
  (if (`self.CurrentWeaponIsMelee?`)
    (`self.MeleeWeaponInHand`
      (:`then`
        (bind _mesh (`Character.Mesh` _ascharacter))
        (`Actor.K2_AttachToComponent` (`self.MainHandEquipment`) _mesh "EquipmentOnBack_MainHand" "SnapToTarget" "SnapToTarget" "SnapToTarget" true)
        (set `self.MeleeWeaponInHand` null)
        (`self.ShieldInHand`
          (:`then`
            (`Actor.K2_AttachToComponent` (`self.OffHandEquipment`) _mesh "EquipmentOnBack_Shield" "SnapToTarget" "SnapToTarget" "SnapToTarget" true :!label _label)
            (set `self.ShieldInHand` null))
          (:`else`
            _)))
      (:`else`
        (`self.ShieldInHand`
          (:`then`
            (goto _label))
          (:`else`
            (bind _mainhandequipment (`self.MainHandEquipment`)
              (:`then`
                (`Actor.K2_AttachToComponent` _mainhandequipment _mesh "RightHandSocket" "SnapToTarget" "SnapToTarget" "SnapToTarget" true)
                (set `self.MeleeWeaponInHand` _mainhandequipment))
              (:`else`
                _))
            (bind _offhandequipment (`self.OffHandEquipment`)
              (:`then`
                (`Actor.K2_AttachToComponent` _offhandequipment _mesh "LeftHandSocket" "SnapToTarget" "SnapToTarget" "SnapToTarget" true)
                (set `self.ShieldInHand` _offhandequipment))
              (:`else`
                _))))))
    (else
      (`self.RangedInHand`
        (:`then`
          (`Actor.K2_AttachToComponent` _rangedequipment _mesh "EquipmentOnBack_Ranged" "SnapToTarget" "SnapToTarget" "SnapToTarget" true)
          (set `self.RangedInHand` null))
        (:`else`
          (bind _rangedequipment_2 (`self.RangedEquipment`)
            (:`then`
              (`Actor.K2_AttachToComponent` _rangedequipment _mesh "LeftHandRangedSocket" "SnapToTarget" "SnapToTarget" "SnapToTarget" true)
              (`Actor.K2_AttachToComponent` _rangedequipment_2 _mesh "LeftHandRangedSocket" "SnapToTarget" "SnapToTarget" "SnapToTarget" true)
              (set `self.RangedInHand` _rangedequipment_2))
            (:`else`
              _))))))
  (`self.GetStance`))

(fn `UnequipItem`
  (params (ItemInfo :type "/Game/SubSystems/Inventory/SystemFiles/S_ItemInfo Structure"))
  (locals (EquipmentToRemove :type "/Game/SubSystems/Inventory/Equipment/BP_EquipmentBasic Object Reference"))
  (bind _equipmenttoremove (`local.EquipmentToRemove`))
  (bind (_datatable _rowname) (break `DataTableRowHandle` (`.EquipmentInfo_38_F72D43004768FCF4953CF38D6FA6EDE3` (break `/Game/SubSystems/Inventory/SystemFiles/S_ItemInfo` ItemInfo))))
  (bind _iteminfo (`/Game/SubSystems/Inventory/Equipment/BP_EquipmentBasic.ItemInfo` _equipmenttoremove))
  (bind _returnvalue (`|GetDataTableRow` _datatable _rowname)
    (:`then`
      (switch `/Game/SubSystems/Inventory/SystemFiles/E_EquipmentSlot` (`.EquipmentSlot_25_A9E74878467C51A95BFF90B42A72CCB3` (break `/Game/SubSystems/Inventory/SystemFiles/S_EquipmentInfo` _returnvalue))
        (:`NewEnumerator0`
          (set `local.EquipmentToRemove` (`self.ArmorEquipment`))
          (set `self.ArmorEquipment` null))
        (:`NewEnumerator1`
          (set `local.EquipmentToRemove` (`self.MainHandEquipment`))
          (set `self.MainHandEquipment` null)
          (set `self.MeleeWeaponInHand` null))
        (:`NewEnumerator2`
          (set `local.EquipmentToRemove` (`self.OffHandEquipment`))
          (set `self.OffHandEquipment` null)
          (set `self.ShieldInHand` null))
        (:`NewEnumerator3`
          (set `local.EquipmentToRemove` (`self.AccessoryEquipment`))
          (set `self.AccessoryEquipment` null))
        (:`NewEnumerator4`
          (set `local.EquipmentToRemove` (`self.RangedEquipment`))
          (set `self.RangedEquipment` null)
          (set `self.RangedInHand` null)))
      (`Actor.K2_DetachFromActor` _equipmenttoremove "KeepRelative" "KeepRelative" "KeepRelative")
      (bind _asbp_player (cast `/Game/Base/BP_Player` (`self.GetOwner`)))
      (`/Game/SubSystems/Inventory/SystemFiles/AC_Inventory.AddToInventory` (`/Game/Base/BP_Player.PlayerInventory` _asbp_player) _iteminfo)
      (`KismetArrayLibrary.Array_RemoveItem` (`self.EquipmentOnCharacter`) _iteminfo)
      (`self.GetStance`))))