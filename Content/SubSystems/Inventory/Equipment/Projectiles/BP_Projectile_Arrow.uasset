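; Arrow projectile that detaches on launch and flies toward its owner's combat target or the camera's aim point.
; Launch takes the AC_CombatSystem target, falling back to a camera line trace, and sets ProjectileMovement velocity from the owner's ArrowSocket toward it.
; Tip overlaps with non-owner static or skeletal meshes, or the mutant training dummy, apply fixed damage and destroy the arrow, with debug print and sphere.
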(event `Launch`
  (bind _projectilemovement (`self.ProjectileMovement`))
  (bind (_returnvalue_location _returnvalue_rotation) (`KismetMathLibrary.BreakTransform` (`self.GetTransform` (`GameplayStatics.GetPlayerCameraManager` 0))))
  (bind _ascharacter (cast `Character` (`self.GetOwner`) :!pure true))
  (`self.K2_DetachFromActor` "KeepWorld" "KeepRelative" "KeepWorld")
  (bind _target (`/Game/SubSystems/Combat/AC_CombatSystem.Target` (`self.GetComponentByClass` _ascharacter "/Game/SubSystems/Combat/AC_CombatSystem.AC_CombatSystem_C"))
    (:`then`
      (set `self.HitTargetLocation` (`self.K2_GetActorLocation` _target)))
    (:`else`
      (bind (_outhit _returnvalue) (`KismetSystemLibrary.LineTraceSingle` :`Start` _returnvalue_location :`End` (+ _returnvalue_location (* (`KismetMathLibrary.GetForwardVector` _returnvalue_rotation) 5000.0)) :`TraceChannel` "TraceTypeQuery1" :`DrawDebugType` "ForDuration"))
      (bind (_bblockinghit _binitialoverlap _time _distance _location _impactpoint _normal _impactnormal _physmat _hitactor _hitcomponent _hitbonename _hititem _elementindex _faceindex _tracestart _traceend) (`GameplayStatics.BreakHitResult` _outhit))
      (set `self.HitTargetLocation` (`KismetMathLibrary.SelectVector` _impactpoint _traceend _returnvalue))))
  (set `MovementComponent.Velocity` (* (`KismetMathLibrary.Normal` (- (`self.HitTargetLocation`) (`SceneComponent.GetSocketLocation` (`Character.Mesh` _ascharacter) "ArrowSocket")) 0.0) (`ProjectileMovementComponent.InitialSpeed` _projectilemovement)) _projectilemovement)
  (`ActorComponent.Activate` _projectilemovement false))

(event `self.ArrowTip.OnComponentBeginOverlap`
  (params (OverlappedComponent :type "PrimitiveComponent Object Reference") (OtherActor :type "Actor Object Reference") (OtherComp :type "PrimitiveComponent Object Reference") (OtherBodyIndex :type Integer) (bFromSweep :type Boolean) (SweepResult :type "HitResult Structure (by ref)"))
  (bind _returnvalue (`self.GetOwner`))
  (if (!= OtherActor _returnvalue)
    (cast `StaticMeshComponent` OtherComp
      (:`then`
        _)
      (:`CastFailed`
        (cast `SkeletalMeshComponent` OtherComp
          (:`then`
            _)
          (:`CastFailed`
            (cast `/Game/NPC/BP_NPC_MutantTrainingDummy` OtherActor)))))
    (`KismetSystemLibrary.PrintString` (`KismetSystemLibrary.GetDisplayName` OtherActor))
    (`GameplayStatics.ApplyDamage` OtherActor 5.0 null _returnvalue)
    (`ActorComponent.Deactivate` (`self.ProjectileMovement`))
    (`KismetSystemLibrary.DrawDebugSphere` (`SceneComponent.K2_GetComponentLocation` (`self.ArrowTip`)) 10.0 36 (struct :`R` 1.0 :`A` 1.0) 5.0 10.0)
    (`self.K2_DestroyActor`)))

(fn `UserConstructionScript`
  (`parent.UserConstructionScript`))