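; BP_ItemBase is the base inventory item that the player can highlight and pick up.
; PickUpItem checks that the item is in the player's range, prints its display name and passes it to the player inventory subsystem.
; HighlightInteractable enables custom depth on the mesh while the item is in range and hit by the player's forward trace, re-checking on a timer.
; GetName returns an empty string.
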(event `/Game/SubSystems/Inventory/Interfaces/BPI_InventoryInteraction.PickUpItem`
  ;[1 1 1] Pick up item, add to player's inventory
  (if (`/Game/Base/BP_Player.QueryItemInRange` (`/Game/Base/BFL_BasicFunctions.GetPlayerCharacter`) self)
    (`KismetSystemLibrary.PrintString` (`KismetSystemLibrary.GetDisplayName` self))
    (`/Game/SubSystems/Inventory/SystemFiles/AC_Inventory.PickUpItem` (`/Game/Base/BFL_BasicFunctions.GetPlayerInventorySubsystem`) self)))

(event `/Game/Base/BPI_Interact.HighlightInteractable`
  (bind _staticmesh (`self.StaticMesh`))
  (if (and (== (`.HitActor` (`GameplayStatics.BreakHitResult` (`/Game/Base/BP_PlayerController.TraceInFrontOfPlayer` (`/Game/Base/BFL_BasicFunctions.GetPlayerController`)))) self) (`/Game/Base/BP_Player.QueryItemInRange` (`/Game/Base/BFL_BasicFunctions.GetPlayerCharacter`) self))
    (`PrimitiveComponent.SetRenderCustomDepth` _staticmesh true)
    (bind _returnvalue (`KismetSystemLibrary.K2_SetTimerDelegate` (delegate `/Game/Base/BPI_Interact.HighlightInteractable`) 0.1 true))
    (else
      (`PrimitiveComponent.SetRenderCustomDepth` _staticmesh false)
      (`KismetSystemLibrary.K2_ClearAndInvalidateTimerHandle` _returnvalue))))

(fn `GetName`
  (returns (Name :type Text))
  (return ""))

(fn `UserConstructionScript`)