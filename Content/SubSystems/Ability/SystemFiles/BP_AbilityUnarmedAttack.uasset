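; Unarmed attack ability that performs a right-hook punch and prints a debug message when it begins play.
; PlayAnimation plays the hook montage on the skeletal mesh supplied by the caller.
; When the montage completes or is interrupted, it sets the player character's movement mode back to Walking, regardless of which mesh played it.
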(event `self.ReceiveBeginPlay`
  (`parent.ReceiveBeginPlay`)
  (`KismetSystemLibrary.PrintString` "Punch!"))

(event `self.PlayAnimation`
  (params (MeshForMontage :type "SkeletalMeshComponent Object Reference"))
  (`|PlayMontage` MeshForMontage "/Game/Mixamo/Animations/Nordstrom/Combat/Action_Right_Hook_Montage.Action_Right_Hook_Montage"
    (:`OnCompleted`
      _)
    (:`OnInterrupted`
      _))
  (`CharacterMovementComponent.SetMovementMode` (`Character.CharacterMovement` (`/Game/Base/BFL_BasicFunctions.GetPlayerCharacter`)) "MOVE_Walking" 0))

(fn `UserConstructionScript`
  (`parent.UserConstructionScript`))