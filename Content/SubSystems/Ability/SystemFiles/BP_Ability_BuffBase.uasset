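; BP_Ability_BuffBase is a base ability actor for buffs, with a CastAbility function triggered through OnNotification.
; On BeginPlay it runs ClearDuplicate, which scans the owner's attached actors for instances of its own class but does nothing with matches.
; CastAbility is empty, and the nodes for destroying duplicates, signalling cleared buffs to player stats and adding the buff to the HUD panel are disconnected.
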(event `self.ReceiveBeginPlay`
  (`parent.ReceiveBeginPlay`)
  (`self.ClearDuplicate`))

(event `self.ReceiveEndPlay`
  (params (EndPlayReason :type "EEndPlayReason Enum" :default "Destroyed")))

(fn `CastAbility`)

(fn `ClearDuplicate`
  (for _array_element (`self.GetAttachedActors` (`self.GetOwner`) true)
    (if (== (`GameplayStatics.GetObjectClass` _array_element) (`GameplayStatics.GetObjectClass` self))
      _)))

(fn `OnNotification`
  (params (NotificationName :type Name :default "None"))
  (switch `name` NotificationName
    (:`CastAbility`
      (`self.CastAbility`))))

(fn `UserConstructionScript`
  (`parent.UserConstructionScript`))