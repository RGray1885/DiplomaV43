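; BP_AbilityKick is the kick ability, a child Blueprint that plays an axe standing-melee kick montage on its owning Character.
; UseStandard runs the parent logic, casts the owner to Character and passes its mesh to PlayAnimation.
; When the montage completes or is interrupted, the player character's movement mode is set to Walking, regardless of which Character owns the ability.
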(event `self.ReceiveBeginPlay`
  (`parent.ReceiveBeginPlay`)
  (`KismetSystemLibrary.PrintString` "Kick"))

(event `PlayAnimation`
  (params (MeshForMontage :type "SkeletalMeshComponent Object Reference"))
  (`|PlayMontage` MeshForMontage "/Game/Mixamo/Animations/Nordstrom/Combat/Axe_StandingMelee_Kick_Montage.Axe_StandingMelee_Kick_Montage"
    (:`OnCompleted`
      _)
    (:`OnInterrupted`
      _))
  (`CharacterMovementComponent.SetMovementMode` (`Character.CharacterMovement` (`/Game/Base/BFL_BasicFunctions.GetPlayerCharacter`)) "MOVE_Walking" 0))

(fn `UserConstructionScript`
  (`parent.UserConstructionScript`))

(fn `UseStandard`
  (`parent.UseStandard`)
  (bind _ascharacter (cast `Character` (`self.GetOwner`)))
  (`self.PlayAnimation` (`Character.Mesh` _ascharacter)))