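; Kick ability actor that flags the player character as kicking for as long as the actor exists.
; BeginPlay runs the parent logic, prints a "Kick" debug string and sets IsKicking on the player character, and EndPlay clears the flag.
; ApplyDamage and the construction script only call their parent versions, adding no kick-specific logic.
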(event `self.ReceiveBeginPlay`
  (`parent.ReceiveBeginPlay`)
  (`KismetSystemLibrary.PrintString` "Kick")
  (set `/Game/Base/BP_Player.IsKicking` true (`/Game/Base/BFL_BasicFunctions.GetPlayerCharacter`)))

(event `self.ReceiveEndPlay`
  (params (EndPlayReason :type "EEndPlayReason Enum" :default "Destroyed"))
  (set `/Game/Base/BP_Player.IsKicking` false (`/Game/Base/BFL_BasicFunctions.GetPlayerCharacter`)))

(fn `ApplyDamage`
  (`parent.ApplyDamage`))

(fn `UserConstructionScript`
  (`parent.UserConstructionScript`))