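; Buff ability Blueprint that temporarily fortifies player stats when cast.
; CastAbility runs the parent cast, activates the particle system and applies the ability effect.
; The effect is passed from AbilityInfo to the player stats subsystem, and a one-shot timer is set for the ability duration.
; When the timer fires, TickBuff removes the fortify bonus, so it acts as expiry rather than a periodic tick.
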(event `self.ReceiveBeginPlay`
  (`parent.ReceiveBeginPlay`))

(event `TickBuff`
  (`/Game/SubSystems/PlayerStats/SystemFiles/AC_CharacterStats.RemoveFortifyBonus` (`/Game/Base/BFL_BasicFunctions.GetPlayerStatsSubsystem`) (`.AbilityEffect_17_9A09C93F49D390455C9DFA863FD069DA` (break `/Game/SubSystems/Ability/SystemFiles/S_AbilityInfo` (`self.AbilityInfo`)))))

(event `ApplyAbilityEffect`
  (bind (_abilityclass _abilityname _abilitydescription _abilitytype _ispassive _abilityeffect _abilityicon _manacost _abilityrange _abilityduration) (break `/Game/SubSystems/Ability/SystemFiles/S_AbilityInfo` (`self.AbilityInfo`)))
  (`/Game/SubSystems/PlayerStats/SystemFiles/AC_CharacterStats.FortifyStats` (`/Game/Base/BFL_BasicFunctions.GetPlayerStatsSubsystem`) _abilityeffect)
  (bind _returnvalue (`KismetSystemLibrary.K2_SetTimerDelegate` (delegate `TickBuff`) _abilityduration))
  (set `self.BuffTimer` _returnvalue))

(fn `CastAbility`
  (`parent.CastAbility`)
  (`ActorComponent.Activate` (`self.ParticleSystem`) false)
  (`self.ApplyAbilityEffect`))

(fn `UserConstructionScript`
  (`parent.UserConstructionScript`))