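; BP_AbilityBase is the base Blueprint for abilities in the ability subsystem.
; On BeginPlay it loads its AbilityInfo from the data table row named by the AbilityDTH handle.
; UseAbility switches on AbilityInfo.AbilityType and calls the matching On Self, On Target, On Area or Standard function.
; Those four functions are empty here, leaving the actual effects unimplemented in this base.
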(event `self.ReceiveBeginPlay`
  (bind (_abilitydth_datatable _abilitydth_rowname) (break `DataTableRowHandle` (`self.AbilityDTH`)))
  (bind _returnvalue (`|GetDataTableRow` _abilitydth_datatable _abilitydth_rowname)
    (:`then`
      (set `self.AbilityInfo` _returnvalue))))

(fn `UseAbility`
  (switch `/Game/SubSystems/Ability/SystemFiles/E_AbilityType` (`.AbilityType_10_9208DFE344939450854AA8BDEE0F0997` (break `/Game/SubSystems/Ability/SystemFiles/S_AbilityInfo` (`self.AbilityInfo`)))
    (:`NewEnumerator0`
      (`self.UseOnSelf`))
    (:`NewEnumerator1`
      (`self.UseOnTarget`))
    (:`NewEnumerator2`
      (`self.UseOnArea`))
    (:`NewEnumerator3`
      (`self.UseStandard`))))

(fn `UseOnArea`)

(fn `UseOnSelf`)

(fn `UseOnTarget`)

(fn `UserConstructionScript`)

(fn `UseStandard`)