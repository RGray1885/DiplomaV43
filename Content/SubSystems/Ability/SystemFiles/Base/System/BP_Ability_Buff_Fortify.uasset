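; A buff ability Blueprint that temporarily fortifies the player's defence.
; Applying the effect casts the owner to BP_Player and calls FortifyDefence on its PlayerStats with the ability's Potency.
; RemoveBuff reverses it through DeFortifyDefence with the same Potency.
; Both overrides then call their parent versions, and both do nothing if the owner is not a BP_Player.
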(fn `ApplyAbilityEffect`
  (bind _asbp_player (cast `/Game/Base/BP_Player` (`self.GetOwner`)))
  (`/Game/SubSystems/PlayerStats/SystemFiles/AC_CharacterStats.FortifyDefence` (`/Game/Base/BP_Player.PlayerStats` _asbp_player) (`.Potency_26_8BFAC47F4AC0A24BF9EC86AE51867DE1` (break `/Game/SubSystems/Ability/SystemFiles/Base/System/S_AbilityDetails` (`self.AbilityDetails`))))
  (`parent.ApplyAbilityEffect`))

(fn `RemoveBuff`
  (bind _asbp_player (cast `/Game/Base/BP_Player` (`self.GetOwner`)))
  (`/Game/SubSystems/PlayerStats/SystemFiles/AC_CharacterStats.DeFortifyDefence` (`/Game/Base/BP_Player.PlayerStats` _asbp_player) (`.Potency_26_8BFAC47F4AC0A24BF9EC86AE51867DE1` (break `/Game/SubSystems/Ability/SystemFiles/Base/System/S_AbilityDetails` (`self.AbilityDetails`))))
  (`parent.RemoveBuff`))

(fn `UserConstructionScript`
  (`parent.UserConstructionScript`))