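; Actor component that manages a character's abilities: learning, slotting, casting and the related skill UI.
; Learning spends ability points from the player stats subsystem, while equipping sets a left or right slot class.
; UseAbility spawns only the right-slot ability actor, gated by stance, no playing montage and enough mana, then drains the cost read from the ability's data table row.
; It also toggles skill book and selection bar widgets on the HUD.
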(event `self.ReceiveBeginPlay`
  (bind _ascharacter (cast `Character` (`self.GetOwner`)))
  (set `self.Owner` _ascharacter))

(event `UseAbility`
  (params (Key :type "Key Structure" :default "None"))
  (bind _rightslotability (`self.RightSlotAbility`))
  (bind _owner (`self.Owner`))
  (bind _returnvalue (`Actor.GetComponentByClass` _owner "/Game/SubSystems/PlayerStats/SystemFiles/AC_CharacterStats.AC_CharacterStats_C"))
  (if (`|EnumInequality` (`/Game/SubSystems/Inventory/SystemFiles/AC_Equipmentv2.CurrentStance` (`Actor.GetComponentByClass` _owner "/Game/SubSystems/Inventory/SystemFiles/AC_Equipmentv2.AC_Equipmentv2_C")) "NewEnumerator3")
    (if (not (`AnimInstance.IsAnyMontagePlaying` (`SkeletalMeshComponent.GetAnimInstance` (`Character.Mesh` _owner))))
      (bind _cost (`self.GetAbilityCost` _rightslotability))
      (if (not (< (- (`/Game/SubSystems/PlayerStats/SystemFiles/AC_CharacterStats.ManaCurrent` _returnvalue) _cost) 0.0))
        (`|SpawnActorFromClass` _rightslotability (`KismetMathLibrary.MakeTransform` (`Actor.K2_GetActorLocation` _owner)) "Undefined" "OverrideRootScale" (`self.Owner`) null)
        (`/Game/SubSystems/PlayerStats/SystemFiles/AC_CharacterStats.DrainMana` _returnvalue _cost)))))

(fn `EquipSkill`
  (params (Skill :type "/Game/SubSystems/Ability/SystemFiles/Base/System/BP_BaseAbility Class Reference") (LeftSlot :type Boolean))
  (if LeftSlot
    (set `self.LeftSlotAbility` Skill)
    (else
      (set `self.RightSlotAbility` Skill))))

(fn `GetAbilityCost`
  (params (Class :type "/Game/SubSystems/Ability/SystemFiles/Base/System/BP_BaseAbility Class Reference"))
  (returns (Cost :type "Float (double-precision)"))
  (bind (_datatable _rowname) (break `DataTableRowHandle` (`.AbilityDetailsDTH` (defaults `Object` Class))))
  (bind _returnvalue (`|GetDataTableRow` _datatable _rowname)
    (:`then`
      _)
    (:`RowNotFound`
      _))
  (return (`.Cost_7_D513DE62409A5965DBDA0C80D48B1178` (break `/Game/SubSystems/Ability/SystemFiles/Base/System/S_AbilityDetails` _returnvalue))))

(fn `LearnSkill`
  (params (Skill :type "/Game/SubSystems/Ability/SystemFiles/Base/System/BP_BaseAbility Class Reference"))
  (bind _abilitypoints (`/Game/SubSystems/PlayerStats/SystemFiles/AC_CharacterStats.AbilityPoints` (`/Game/Base/BFL_BasicFunctions.GetPlayerStatsSubsystem`)))
  (if (> _abilitypoints 0)
    (bind _alreadylearned (`self.QueryLearnedSkill` Skill))
    (if _alreadylearned
      (`KismetSystemLibrary.PrintString` "Already learned")
      (else
        (`KismetArrayLibrary.Array_AddUnique` (`self.AbilitiesAvailable`) Skill)
        (`KismetSystemLibrary.PrintString` (`KismetStringLibrary.Concat_StrStr` (`KismetSystemLibrary.GetClassDisplayName` Skill) " learned"))
        (`/Engine/EditorBlueprintResources/StandardMacros.DecrementInt` _abilitypoints)))
    (else
      (`KismetSystemLibrary.PrintString` "Not enough ability points"))))

(fn `OpenSkillBook`
  (bind _skillbookref (`self.SkillBookRef`)
    (:`then`
      (`Widget.RemoveFromParent` _skillbookref)
      (set `self.SkillBookRef` null))
    (:`else`
      (bind _returnvalue (`|CreateWidget` "/Game/SubSystems/Ability/SystemFiles/Base/UI/WBP_SkillBook.WBP_SkillBook_C"))
      (bind _output_get (set `self.SkillBookRef` _returnvalue))
      (bind _returnvalue_2 (`CanvasPanel.AddChildToCanvas` (`/Game/Base/WBP_Player_UI.SkillBookCanvas` (`/Game/Base/BP_Player_HUD.PlayerUI_Ref` (`/Game/Base/BFL_BasicFunctions.Get Player HUD`))) _output_get))
      (`CanvasPanelSlot.SetAutoSize` _returnvalue_2 true))))

(fn `OpenSkillSelector`
  (params (PressedIcon :type "/Game/SubSystems/Ability/SystemFiles/Base/UI/WBP_AbilityIcon Object Reference"))
  (bind _skillselector (`self.SkillSelector`)
    (:`then`
      (`Widget.RemoveFromParent` _skillselector)
      (set `self.SkillSelector` null))
    (:`else`
      (bind _returnvalue (`|CreateWidget` "/Game/SubSystems/Ability/SystemFiles/Base/UI/WBP_SkillSelectionBar.WBP_SkillSelectionBar_C" null (`/Game/SubSystems/Ability/SystemFiles/Base/UI/WBP_AbilityIcon.LeftSlot` PressedIcon)))
      (bind _output_get (set `self.SkillSelector` _returnvalue))
      (bind _returnvalue_2 (`CanvasPanel.AddChildToCanvas` (`/Game/Base/WBP_Player_UI.SkillSelector` (`/Game/Base/BP_Player_HUD.PlayerUI_Ref` (`/Game/Base/BFL_BasicFunctions.Get Player HUD`))) _output_get))
      (`CanvasPanelSlot.SetAutoSize` _returnvalue_2 true))))

(fn `QueryLearnedSkill`
  (params (Skill :type "/Game/SubSystems/Ability/SystemFiles/Base/System/BP_BaseAbility Class Reference"))
  (returns (AlreadyLearned :type Boolean))
  (return (`KismetArrayLibrary.Array_Contains` (`self.AbilitiesAvailable`) Skill)))