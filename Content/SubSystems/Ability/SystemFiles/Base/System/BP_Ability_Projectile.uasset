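; Base projectile ability actor that is cast from the owner's hand and damages on hitting an enemy.
; The equipment state picks the cast montage and hand socket to attach to, then a montage notify detaches the actor and activates projectile movement.
; Overlapping an "Enemy"-tagged actor swaps in an explosion effect, draws debug output and damages every overlapping actor with random player damage scaled by Potency.
; Lifespan comes from the ability's duration.
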(event `self.ReceiveBeginPlay`
  (`parent.ReceiveBeginPlay`)
  (`self.SetLifeSpan` (`.Duration_11_F5B6C96A46D703A021A132921AFE7BD3` (break `/Game/SubSystems/Ability/SystemFiles/Base/System/S_AbilityDetails` (`self.AbilityDetails`)))))

(event `self.ProjectileCollision.OnComponentBeginOverlap`
  (params (OverlappedComponent :type "PrimitiveComponent Object Reference") (OtherActor :type "Actor Object Reference") (OtherComp :type "PrimitiveComponent Object Reference") (OtherBodyIndex :type Integer) (bFromSweep :type Boolean) (SweepResult :type "HitResult Structure (by ref)"))
  (if (`self.ActorHasTag` OtherActor "Enemy")
    (`KismetSystemLibrary.PrintString` (`KismetSystemLibrary.GetDisplayName` OtherActor))
    (`KismetSystemLibrary.DrawDebugSphere` (`self.K2_GetActorLocation` OtherActor) 100.0 12 (struct :`R` 1.0 :`G` 0.22198 :`B` 0.031642 :`A` 1.0) 5.0 10.0)
    (`ParticleSystemComponent.SetTemplate` (`self.ParticleSystem`) "/Game/Assets/FXVarietyPack/Particles/P_ky_explosion.P_ky_explosion")
    (`self.ApplyAbilityEffect`)))

(fn `ApplyAbilityEffect`
  (bind _playerstats (`/Game/Base/BFL_BasicFunctions.GetPlayerStatsSubsystem`))
  (bind (_abilitydetails_class _abilitydetails_name _abilitydetails_description _abilitydetails_cost _abilitydetails_duration _abilitydetails_isinterruptable _abilitydetails_requierstarget _abilitydetails_icon _abilitydetails_potency) (break `/Game/SubSystems/Ability/SystemFiles/Base/System/S_AbilityDetails` (`self.AbilityDetails`)))
  (for _array_element (`PrimitiveComponent.GetOverlappingActors` (`self.ProjectileCollision`) null)
    (`GameplayStatics.ApplyDamage` _array_element (* (`KismetMathLibrary.RandomFloatInRange` (`/Game/SubSystems/PlayerStats/SystemFiles/AC_CharacterStats.DamageMin` _playerstats) (`/Game/SubSystems/PlayerStats/SystemFiles/AC_CharacterStats.DamageMax` _playerstats)) _abilitydetails_potency) null (`self.GetOwner`)))
  (`parent.ApplyAbilityEffect`))

(fn `AttachToSocket`
  (bind (_swordandshield _twohanded _poseonehand _poseunarmed) (`/Game/SubSystems/Inventory/SystemFiles/AC_EquipmentComponent.GetEquipmentState` (`/Game/Base/BFL_BasicFunctions.GetPlayerEquipmentSubsystem`)))
  (if _poseunarmed
    (set `self.AbilityCastMontage` "/Game/Mixamo/Animations/Nordstrom/Cast/Standing_1H_Magic_Attack_01_Montage.Standing_1H_Magic_Attack_01_Montage")
    (set `self.SocketToAttach` "RightHandCastSocket")
    (else
      (if _swordandshield
        (set `self.AbilityCastMontage` "/Game/Mixamo/Animations/Nordstrom/Cast/Sword_And_Shield_Casting_Single_M.Sword_And_Shield_Casting_Single_M")
        (else
          (set `self.AbilityCastMontage` "/Game/Mixamo/Animations/Nordstrom/Cast/GreatSword1HCast_Montage.GreatSword1HCast_Montage")))
      (set `self.SocketToAttach` "LeftHandCastSocket")))
  (bind _ascharacter (cast `Character` (`self.GetOwner`)))
  (`self.K2_AttachToComponent` self (`Character.Mesh` _ascharacter) (`self.SocketToAttach`) "SnapToTarget" "SnapToTarget" "SnapToTarget" true))

(fn `LaunchProjectile`
  (`self.K2_DetachFromActor` "KeepWorld" "KeepWorld" "KeepWorld")
  (`ActorComponent.Activate` (`self.ProjectileMovement`) false))

(fn `OnNotifyBegin`
  (params (NotifyName :type Name))
  (`parent.OnNotifyBegin` NotifyName)
  (switch `name` NotifyName
    (:`LaunchProjectile`
      (`self.LaunchProjectile`))))

(fn `UserConstructionScript`
  (`parent.UserConstructionScript`))