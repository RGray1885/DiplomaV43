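; Base area-of-effect ability actor that starts as an effect in the player's casting hand and is left on the ground.
; AttachToSocket snaps it to the right-hand cast socket in the Sword and Shield stance.
; Animation notifies drive the phases: one activates the hand emitter, the other detaches, line-traces for ground placement, and swaps to ground emitter and decal.
; It then calls ApplyAbilityEffect, an empty hook here, and expires after the ability's duration.
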(fn `ActivateHandEmitter`
  (`ActorComponent.Activate` (`self.InHand`) false))

(fn `ApplyAbilityEffect`)

(fn `AttachToSocket`
  (switch `/Game/SubSystems/Inventory/SystemFiles/E_Stance` (`/Game/SubSystems/Inventory/SystemFiles/AC_Equipmentv2.CurrentStance` (`/Game/Base/BP_Player.PlayEquipment` (`/Game/Base/BFL_BasicFunctions.GetPlayerCharacter`)))
    (:`NewEnumerator4`
      (set `self.SocketToAttach` "RightHandCastSocket")
      (`self.K2_AttachToComponent` self (`Character.Mesh` (`/Game/Base/BFL_BasicFunctions.GetPlayerCharacter`)) (`self.SocketToAttach`) "SnapToTarget" "SnapToTarget" "SnapToTarget" true))))

(fn `OnNotifyBegin`
  (params (NotifyName :type Name))
  (bind (_abilitydetails_class _abilitydetails_name _abilitydetails_description _abilitydetails_cost _abilitydetails_duration) (break `/Game/SubSystems/Ability/SystemFiles/Base/System/S_AbilityDetails` (`self.AbilityDetails`)))
  (bind _returnvalue (`self.K2_GetActorLocation` (`/Game/Base/BFL_BasicFunctions.GetPlayerCharacter`)))
  (`parent.OnNotifyBegin` NotifyName)
  (switch `name` NotifyName
    (:`SpawnInHand`
      (`self.ActivateHandEmitter`))
    (:`LeaveOnGround`
      (`self.K2_DetachFromActor` "KeepWorld" "KeepRelative" "KeepWorld")
      (bind _outhit (`KismetSystemLibrary.LineTraceSingleForObjects` _returnvalue (+ _returnvalue (- _returnvalue (0.0 0.0 1000.0))) (`|MakeArray` "ObjectTypeQuery1" :!type "EObjectTypeQuery Enum") false (`|MakeArray` (`self.GetOwner`))))
      (`self.K2_SetActorLocation` (`.Location` (`GameplayStatics.BreakHitResult` _outhit)))
      (`ActorComponent.Deactivate` (`self.InHand`))
      (`ActorComponent.Activate` (`self.OnGround`) false)
      (`SceneComponent.SetVisibility` (`self.Decal`) true false)
      (`self.ApplyAbilityEffect`)
      (`self.SetLifeSpan` _abilitydetails_duration))))

(fn `UserConstructionScript`
  (`parent.UserConstructionScript`))