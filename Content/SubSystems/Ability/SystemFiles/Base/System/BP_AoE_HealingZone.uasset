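; Area-of-effect healing zone ability that periodically restores health to players standing inside it.
; ApplyAbilityEffect heals each BP_Player overlapping AreaOfEffect, scaling the amount by that player's own Vitality and Energy and the ability's Potency, rounded up.
; It then sets a looping half-second timer on itself to repeat the pulse.
; The event graph is unused, so the first call comes from outside this graph.
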(fn `ApplyAbilityEffect`
  (for _array_element (`PrimitiveComponent.GetOverlappingActors` (`self.AreaOfEffect`) null)
    (bind _asbp_player (cast `/Game/Base/BP_Player` _array_element))
    (bind _playerstats (`/Game/Base/BP_Player.PlayerStats` _asbp_player))
    (`/Game/SubSystems/PlayerStats/SystemFiles/AC_CharacterStats.RestoreHealth` _playerstats (`KismetMathLibrary.FCeil` (* (+ (`/Game/SubSystems/PlayerStats/SystemFiles/AC_CharacterStats.Vitality` _playerstats) (`/Game/SubSystems/PlayerStats/SystemFiles/AC_CharacterStats.Energy` _playerstats)) (`.Potency_26_8BFAC47F4AC0A24BF9EC86AE51867DE1` (break `/Game/SubSystems/Ability/SystemFiles/Base/System/S_AbilityDetails` (`self.AbilityDetails`)))))))
  (`/Engine/EditorBlueprintResources/StandardMacros.IsValid` self
    (:`Is Valid`
      (`KismetSystemLibrary.K2_SetTimer` null "ApplyAbilityEffect" 0.5 true))))

(fn `UserConstructionScript`
  (`parent.UserConstructionScript`))