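; Player attack ability that plays an equipment-specific animation and damages what it hits.
; On cast it attaches to a socket, picks a random montage for the equipped weapon pose and plays it unless another montage is running.
; Montage notifies apply the effect: a debug-drawn capsule trace from the player to the ability subsystem's location.
; The hit actor takes rolled stat damage plus ability potency; montage completion or blend-out completes the cast.
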(event `self.BeginCasting`
  (bind _mesh (`Character.Mesh` (`/Game/Base/BFL_BasicFunctions.GetPlayerCharacter`)))
  (`self.AttachToSocket`)
  (`KismetSystemLibrary.PrintString` "Casting")
  (`self.SelectMontageToPlay`)
  (if (not (`AnimInstance.IsAnyMontagePlaying` (`SkeletalMeshComponent.GetAnimInstance` _mesh)))
    (bind _notifyname (`|PlayMontage` _mesh (`self.AbilityCastMontage`))
      (:`OnCompleted`
        (`self.CastComplete` :!label _label)
        (`KismetSystemLibrary.PrintString` "Complete"))
      (:`OnBlendOut`
        (goto _label))
      (:`OnInterrupted`
        (`KismetSystemLibrary.PrintString` "Interrupted"))
      (:`OnNotifyBegin`
        (`self.OnNotifyBegin` _notifyname)))))

(fn `ApplyAbilityEffect`
  (locals (ClickLocation :type "Vector Structure" :default (0.0 0.0 0.0)))
  (bind _playerstats (`/Game/Base/BFL_BasicFunctions.GetPlayerStatsSubsystem`))
  (bind _playercharacter (`/Game/Base/BFL_BasicFunctions.GetPlayerCharacter`))
  (bind (_abilitydetails_class _abilitydetails_name _abilitydetails_description _abilitydetails_cost _abilitydetails_duration _abilitydetails_isinterruptable _abilitydetails_requierstarget _abilitydetails_icon _abilitydetails_potency) (break `/Game/SubSystems/Ability/SystemFiles/Base/System/S_AbilityDetails` (`self.AbilityDetails`)))
  (`parent.ApplyAbilityEffect`)
  (bind _outhit (`KismetSystemLibrary.CapsuleTraceSingle` (`self.K2_GetActorLocation` _playercharacter) (`/Game/SubSystems/Ability/SystemFiles/Base/System/AC_AbilitySystemComponent.Location` (`/Game/Base/BFL_BasicFunctions.GetPlayerAbilitySubsystem`)) 60.0 20.0 "TraceTypeQuery1" false (`|MakeArray` _playercharacter :!type "Actor Object Reference") "ForDuration"))
  (`GameplayStatics.ApplyDamage` (`.HitActor` (`GameplayStatics.BreakHitResult` _outhit)) (+ (`KismetMathLibrary.Conv_IntToDouble` (`KismetMathLibrary.FCeil` (`KismetMathLibrary.RandomFloatInRange` (`/Game/SubSystems/PlayerStats/SystemFiles/AC_CharacterStats.DamageMin` _playerstats) (`/Game/SubSystems/PlayerStats/SystemFiles/AC_CharacterStats.DamageMax` _playerstats)))) _abilitydetails_potency) null _playercharacter))

(fn `OnNotifyBegin`
  (params (NotifyName :type Name))
  (`parent.OnNotifyBegin` NotifyName)
  (switch `name` NotifyName
    (:`ApplyEffect`
      (`self.ApplyAbilityEffect`))))

(fn `SelectMontageToPlay`
  (bind (_swordandshield _twohanded _poseonehand _poseunarmed) (`/Game/SubSystems/Inventory/SystemFiles/AC_EquipmentComponent.GetEquipmentState` (`/Game/Base/BFL_BasicFunctions.GetPlayerEquipmentSubsystem`)))
  (if _swordandshield
    (set `self.AbilityCastMontage` (`KismetArrayLibrary.Array_Random` (`self.SwordShieldMontages`)))
    (elif _twohanded
      (set `self.AbilityCastMontage` (`KismetArrayLibrary.Array_Random` (`self.TwoHandedMontages`)))
      (elif _poseonehand
        (set `self.AbilityCastMontage` (`KismetArrayLibrary.Array_Random` (`self.OneHandMontages`)))
        (elif _poseunarmed
          (set `self.AbilityCastMontage` (`KismetArrayLibrary.Array_Random` (`self.UnarmedMontages`))))))))

(fn `UserConstructionScript`
  (`parent.UserConstructionScript`))