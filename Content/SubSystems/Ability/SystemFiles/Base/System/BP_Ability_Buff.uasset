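; Buff ability actor that applies an effect to its owner and shows it in the player's HUD buff panel.
; On BeginPlay it destroys actors of the same class attached to the owner to clear duplicates.
; Animation notifies drive effect application, UI registration and cast completion.
; It also provides socket attachment to the owning Character's mesh, and EndPlay calls RemoveBuff to destroy the actor.
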(event `self.ReceiveBeginPlay`
  (`parent.ReceiveBeginPlay`)
  (`self.ClearDuplicate`))

(event `self.ReceiveEndPlay`
  (params (EndPlayReason :type "EEndPlayReason Enum" :default "Destroyed"))
  (`self.RemoveBuff`))

(fn `AttachToSocket`
  (bind _ascharacter (cast `Character` (`self.GetOwner`)))
  (`self.K2_AttachToComponent` self (`Character.Mesh` _ascharacter) (`self.SocketToAttach`) "SnapToTarget" "SnapToTarget" "SnapToTarget" true))

(fn `ClearDuplicate`
  (for _array_element (`self.GetAttachedActors` (`self.GetOwner`) true)
    (if (== (`GameplayStatics.GetObjectClass` _array_element) (`GameplayStatics.GetObjectClass` self))
      (`self.K2_DestroyActor` _array_element)
      (`KismetSystemLibrary.PrintString` "DupeRemoved"))))

(fn `OnNotifyBegin`
  (params (NotifyName :type Name))
  (`parent.OnNotifyBegin` NotifyName)
  (switch `name` NotifyName
    (:`ApplyEffect`
      (`KismetSystemLibrary.PrintString` "Applying Effect")
      (`self.ApplyAbilityEffect`)
      (`/Game/SubSystems/Ability/SystemFiles/Base/UI/WBP_BuffPanelV2.AddBuffToUI` (`/Game/Base/WBP_Player_UI.WBP_BuffPanelV2` (`/Game/Base/BP_Player_HUD.PlayerUI_Ref` (`/Game/Base/BFL_BasicFunctions.Get Player HUD`))) self))
    (:`CastComplete`
      (`self.CastComplete`))))

(fn `RemoveBuff`
  (`self.K2_DestroyActor`))

(fn `UserConstructionScript`
  (`parent.UserConstructionScript`))