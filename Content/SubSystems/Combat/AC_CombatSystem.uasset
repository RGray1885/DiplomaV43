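; Combat component for a Character owner that handles attack, block and target lock-on.
; Attacks play montages chosen by the stance from the Equipment component, with blocking diverting to a sword-and-shield hilt strike.
; Bow attacks spawn an arrow at a socket on a montage notify and use a DoOnce on button release in the launch sequence.
; Lock-on toggles a target found by camera-direction sphere trace, and Tick turns control rotation toward it.
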(event `self.ReceiveBeginPlay`
  (bind _ascharacter (cast `Character` (`self.GetOwner`)))
  (bind _output_get (set `self.OwnerChar` _ascharacter))
  (set `self.Equipment` (`Actor.GetComponentByClass` _output_get "/Game/SubSystems/Inventory/SystemFiles/AC_Equipmentv2.AC_Equipmentv2_C")))

(event `Block`
  (params (ButtonDown :type Boolean))
  (if ButtonDown
    (set `self.IsBlocking` true)
    (else
      (set `self.IsBlocking` false))))

(event `Attack`
  (params (ButtonDown :type Boolean))
  (bind _mesh (`Character.Mesh` (`self.OwnerChar`)))
  (bind _mesh_2 (`Character.Mesh` (`self.OwnerChar`)))
  (if ButtonDown
    (if (`self.IsBlocking`) :!label _label
      (`self.AttackFromBlock`)
      (else
        (switch `/Game/SubSystems/Inventory/SystemFiles/E_Stance` (`/Game/SubSystems/Inventory/SystemFiles/AC_Equipmentv2.CurrentStance` (`self.Equipment`))
          (:`NewEnumerator0`
            (`|PlayMontage` _mesh "/Game/Mannequin/Animations/GreatSword/GreatSword_SlashCombo_Montage.GreatSword_SlashCombo_Montage"))
          (:`NewEnumerator1`
            (`|PlayMontage` _mesh "/Game/Mannequin/Animations/Axe/Axe_Combo3strikes_Montage.Axe_Combo3strikes_Montage"))
          (:`NewEnumerator2`
            (`|PlayMontage` _mesh "/Game/Mannequin/Animations/Bow/BowFireSequence.BowFireSequence"
              (:`then`
                (goto _label_2 :!via `Reset`))
              (:`OnNotifyBegin`
                (bind _rangedinhand (`/Game/SubSystems/Inventory/SystemFiles/AC_Equipmentv2.RangedInHand` (stale _equipment)))
                (bind _returnvalue (`|SpawnActorFromClass` "/Game/SubSystems/Inventory/Equipment/Projectiles/BP_Projectile_Arrow.BP_Projectile_Arrow_C" (`KismetMathLibrary.MakeTransform` (`SceneComponent.GetSocketLocation` _mesh_2 "ArrowSocket") (`SceneComponent.GetSocketRotation` (`/Game/SubSystems/Inventory/Equipment/BP_EquipmentBasic.SkeletalMesh` _rangedinhand) "ArrowSocket")) "Undefined" "OverrideRootScale" (`self.OwnerChar`) (struct) null))
                (bind _output_get (set `self.ArrowProjectile` _returnvalue))
                (`Actor.K2_AttachToComponent` _output_get _mesh_2 "ArrowSocket" "SnapToTarget" "SnapToTarget" "SnapToTarget" true))))
          (:`NewEnumerator3`
            (`|PlayMontage` _mesh "/Game/Mannequin/Animations/Hook_1__UE_Montage.Hook_1__UE_Montage" 1.5))
          (:`NewEnumerator4`
            (`|PlayMontage` _mesh "/Game/Animations/SwordAndShieldAttack_UE_Montage.SwordAndShieldAttack_UE_Montage")))))
    (else
      (bind _equipment (`self.Equipment`)
        (:`then`
          (bind _weaponinhand1 (`/Game/SubSystems/Inventory/SystemFiles/AC_Equipmentv2.GetWeaponInHand` _equipment))
          (`/Engine/EditorBlueprintResources/StandardMacros.IsValid` _weaponinhand1
            (:`Is Valid`
              (if (== _weaponinhand1 _rangedinhand)
                (`/Engine/EditorBlueprintResources/StandardMacros.DoOnce` false :!label _label_2
                  (:`Completed`
                    (`|PlayMontage` _mesh "/Game/Mannequin/Animations/Bow/BowFireSequence.BowFireSequence" 1.0 0.0 "BowOverdrawn"
                      (:`then`
                        (`/Game/SubSystems/Inventory/Equipment/Projectiles/BP_Projectile_Arrow.Launch` (`self.ArrowProjectile`))))))))))
        (:`else`
          (goto _label))))))

(event `AttackFromBlock`
  (if (not (`self.IsAttacking`))
    (switch `/Game/SubSystems/Inventory/SystemFiles/E_Stance` (`/Game/SubSystems/Inventory/SystemFiles/AC_Equipmentv2.CurrentStance` (`self.Equipment`))
      (:`NewEnumerator4`
        (`|PlayMontage` (`Character.Mesh` (`self.OwnerChar`)) "/Game/Mannequin/Animations/SwordAndShield/SwordAndShield_HiltAttack_Montage.SwordAndShield_HiltAttack_Montage")))))

(event `LockOnTarget`
  (bind _returnvalue (`Actor.K2_GetActorLocation` (`self.OwnerChar`)))
  (`self.Target`
    (:`then`
      (set `self.Target` null))
    (:`else`
      (bind (_outhit _returnvalue_2) (`KismetSystemLibrary.SphereTraceSingleForObjects` :`Start` _returnvalue :`End` (+ _returnvalue (* (`KismetMathLibrary.GetForwardVector` (`Actor.K2_GetActorRotation` (`GameplayStatics.GetPlayerCameraManager` 0))) 1000.0)) :`Radius` 128.0 :`ObjectTypes` (`|MakeArray` "ObjectTypeQuery3" :!type "EObjectTypeQuery Enum") :`DrawDebugType` "ForDuration"))
      (if _returnvalue_2
        (bind (_bblockinghit _binitialoverlap _time _distance _location _impactpoint _normal _impactnormal _physmat _hitactor) (`GameplayStatics.BreakHitResult` _outhit))
        (set `self.Target` _hitactor)
        (`KismetSystemLibrary.PrintString` (`KismetSystemLibrary.GetDisplayName` _hitactor))))))

(event `self.ReceiveTick`
  (params (DeltaSeconds :type "Float (single-precision)"))
  (bind _target (`self.Target`)
    (:`then`
      (`Controller.SetControlRotation` (`/Game/Base/BFL_BasicFunctions.GetPlayerController`) (`KismetMathLibrary.FindLookAtRotation` (`Actor.K2_GetActorLocation` (`self.OwnerChar`)) (`Actor.K2_GetActorLocation` _target))))
    (:`else`)))