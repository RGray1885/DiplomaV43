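; BP_BasicContainer is an interactable container that highlights when targeted and opens its trade screen through ACContainer.
; HighlightInteractable enables custom depth on Lid and Box while the player's trace hits it within range, re-checking on a looping timer.
; Interact alternately plays and reverses a timeline that pitches the lid, ignoring input mid-animation.
; When the timeline finishes, it toggles the opened state, showing the trade screen only after opening.
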(event `/Game/Base/BPI_Interact.HighlightInteractable`
  (bind _lid (`self.Lid`))
  (bind _box (`self.Box`))
  (if (and (== (`.HitActor` (`GameplayStatics.BreakHitResult` (`/Game/Base/BP_PlayerController.TraceInFrontOfPlayer` (`/Game/Base/BFL_BasicFunctions.GetPlayerController`)))) self) (`/Game/Base/BP_Player.QueryItemInRange` (`/Game/Base/BFL_BasicFunctions.GetPlayerCharacter`) self))
    (`PrimitiveComponent.SetRenderCustomDepth` _lid true)
    (`PrimitiveComponent.SetRenderCustomDepth` _box true)
    (bind _returnvalue (`KismetSystemLibrary.K2_SetTimerDelegate` (delegate `/Game/Base/BPI_Interact.HighlightInteractable`) 0.1 true))
    (else
      (`PrimitiveComponent.SetRenderCustomDepth` _lid false)
      (`PrimitiveComponent.SetRenderCustomDepth` _box false)
      (`KismetSystemLibrary.K2_ClearAndInvalidateTimerHandle` _returnvalue))))

(event `/Game/Base/BPI_Interact.Interact`
  (bind _lid (`self.Lid`))
  (bind (_returnvalue_roll _returnvalue_pitch _returnvalue_yaw) (`KismetMathLibrary.BreakRotator` (`SceneComponent.K2_GetComponentRotation` _lid)))
  (if (not (`self.ContainerOpening`))
    (set `self.ContainerOpening` true)
    (`/Engine/EditorBlueprintResources/StandardMacros.FlipFlop`
      (:`A`
        (bind (_direction _newtrack_0) (`Timeline|Timeline_0` :!via `PlayFromStart` :!label _label)
          (:`Update`
            (`SceneComponent.K2_SetWorldRotation` _lid (`KismetMathLibrary.MakeRotator` _returnvalue_roll (`KismetMathLibrary.Lerp` 0.0 (`self.RotAngle`) _newtrack_0) _returnvalue_yaw) false false))
          (:`Finished`
            (if (`self.ContainerOpened`)
              (set `self.ContainerOpened` false)
              (else
                (`/Game/SubSystems/Inventory/SystemFiles/AC_Container.OpenTradeScreen` (`self.AC_Container`))
                (set `self.ContainerOpened` true)))
            (set `self.ContainerOpening` false))))
      (:`B`
        (goto _label :!via `ReverseFromEnd`)))))

(fn `GetName`
  (returns (Name :type Text))
  (return "Container"))

(fn `UserConstructionScript`)