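; BP_BasicDoor is an interactable door, named "Door", that swings open and closed on alternate interactions.
; Interact uses a FlipFlop to play or reverse a timeline that lerps the door's world yaw between zero and RotAngle, preserving roll and pitch.
; The DoorOpening flag blocks further interaction until the timeline finishes.
; The yaw is absolute in world space, so the door's placed rotation is not taken into account.
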(event `/Game/Base/BPI_Interact.Interact`
  (bind _door (`self.Door`))
  (bind (_returnvalue_roll _returnvalue_pitch) (`KismetMathLibrary.BreakRotator` (`SceneComponent.K2_GetComponentRotation` _door)))
  (if (not (`self.DoorOpening`))
    (set `self.DoorOpening` true)
    (`/Engine/EditorBlueprintResources/StandardMacros.FlipFlop`
      (:`A`
        (bind (_direction _newtrack_0) (`Timeline|Timeline_0` :!label _label)
          (:`Update`
            (`SceneComponent.K2_SetWorldRotation` _door (`KismetMathLibrary.MakeRotator` _returnvalue_roll _returnvalue_pitch (`KismetMathLibrary.Lerp` 0.0 (`self.RotAngle`) _newtrack_0)) false false))
          (:`Finished`
            (set `self.DoorOpening` false))))
      (:`B`
        (goto _label :!via `Reverse`)))))

(fn `GetName`
  (returns (Name :type Text))
  (return "Door"))

(fn `UserConstructionScript`)