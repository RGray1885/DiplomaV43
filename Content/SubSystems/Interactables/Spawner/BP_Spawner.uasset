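; Interactable lever spawner that replaces its previously spawned character with a new one at an offset from the lever base.
; Interact animates the lever with a timeline, guarded by a Spawning flag and DoOnce.
; Each new character is tagged "Training Gear" and has its AI controller started.
; Highlighting uses custom depth, rechecked on a looping timer while the player targets it within range.
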(event `/Game/Base/BPI_Interact.Interact`
  (if (not (`self.Spawning`))
    (`|ExecutionSequence`
      (:`then_0`
        (goto _label_2 :!via `Reset`))
      (:`then_1`
        (set `self.Spawning` true)
        (bind (_direction _newtrack_0) (`Timeline|Timeline_0` :!label _label)
          (:`Update`
            (`SceneComponent.K2_SetRelativeRotation` (`self.Lever`) (`KismetMathLibrary.MakeRotator` 0.0 (`KismetMathLibrary.Lerp` 360.0 (`self.LeverAngle`) _newtrack_0)) false false))
          (:`Finished`
            (`/Engine/EditorBlueprintResources/StandardMacros.DoOnce` false :!label _label_2
              (:`Completed`
                (set `self.Spawning` false)
                (`KismetSystemLibrary.PrintString` "Spawner")
                (bind _spawnedchar (`self.SpawnedChar`)
                  (:`then`
                    (`self.K2_DestroyActor` _spawnedchar))
                  (:`else`
                    _))
                (bind _returnvalue (`|SpawnActorFromClass` (`self.CharToSpawn`) (`KismetMathLibrary.MakeTransform` (+ (`SceneComponent.K2_GetComponentLocation` (`self.LeverBase`)) (`self.SpawnLocation`))) "Undefined" "OverrideRootScale" null null))
                (bind _output_get (set `self.SpawnedChar` _returnvalue))
                (set `/Game/NPC/BP_NPC_Base.NPCType` "Training Gear" _output_get)
                (bind _asbp_aicontroller (cast `/Game/NPC/AI/BP_AIController` (`Pawn.GetController` _output_get)))
                (`/Game/NPC/AI/BP_AIController.Start` _asbp_aicontroller)
                (goto _label :!via `Reverse`)))))))))

(event `/Game/Base/BPI_Interact.HighlightInteractable`
  (bind _leverbase (`self.LeverBase`))
  (if (and (== (`.HitActor` (`GameplayStatics.BreakHitResult` (`/Game/Base/BP_PlayerController.TraceInFrontOfPlayer` (`/Game/Base/BFL_BasicFunctions.GetPlayerController`)))) self) (`/Game/Base/BP_Player.QueryItemInRange` (`/Game/Base/BFL_BasicFunctions.GetPlayerCharacter`) self))
    (`PrimitiveComponent.SetRenderCustomDepth` _leverbase true)
    (bind _returnvalue (`KismetSystemLibrary.K2_SetTimerDelegate` (delegate `/Game/Base/BPI_Interact.HighlightInteractable`) 0.1 true))
    (else
      (`PrimitiveComponent.SetRenderCustomDepth` _leverbase false)
      (`KismetSystemLibrary.K2_ClearAndInvalidateTimerHandle` _returnvalue))))

(fn `GetName`
  (returns (Name :type Text))
  (return "Spawner"))

(fn `UserConstructionScript`)