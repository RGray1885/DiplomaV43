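; BP_Spawner is an interactable that spawns an AI-controlled training NPC.
; Interact destroys the previously spawned character, spawns CharToSpawn at an offset from the spawner, sets its NPC type to "Training Gear" and starts its BP_AIController.
; HighlightInteractable enables custom-depth highlighting while the player's trace hits the spawner within range, rechecking on a looping timer until that stops.
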(event `/Game/Base/BPI_Interact.Interact`
  (`KismetSystemLibrary.PrintString` "Spawner")
  (bind _spawnedchar (`self.SpawnedChar`)
    (:`then`
      (`self.K2_DestroyActor` _spawnedchar))
    (:`else`
      _))
  (bind _returnvalue (`|SpawnActorFromClass` (`self.CharToSpawn`) (`KismetMathLibrary.MakeTransform` (+ (`self.K2_GetActorLocation`) (`self.SpawnLocation`))) "Undefined" "OverrideRootScale" null null))
  (bind _output_get (set `self.SpawnedChar` _returnvalue))
  (set `/Game/NPC/BP_NPC_Base.NPCType` "Training Gear" _output_get)
  (bind _asbp_aicontroller (cast `/Game/NPC/AI/BP_AIController` (`Pawn.GetController` _output_get)))
  (`/Game/NPC/AI/BP_AIController.Start` _asbp_aicontroller))

(event `/Game/Base/BPI_Interact.HighlightInteractable`
  (bind _staticmesh (`self.StaticMesh`))
  (if (and (== (`.HitActor` (`GameplayStatics.BreakHitResult` (`/Game/Base/BP_PlayerController.TraceInFrontOfPlayer` (`/Game/Base/BFL_BasicFunctions.GetPlayerController`)))) self) (`/Game/Base/BP_Player.QueryItemInRange` (`/Game/Base/BFL_BasicFunctions.GetPlayerCharacter`) self))
    (`PrimitiveComponent.SetRenderCustomDepth` _staticmesh true)
    (bind _returnvalue (`KismetSystemLibrary.K2_SetTimerDelegate` (delegate `/Game/Base/BPI_Interact.HighlightInteractable`) 0.1 true))
    (else
      (`PrimitiveComponent.SetRenderCustomDepth` _staticmesh false)
      (`KismetSystemLibrary.K2_ClearAndInvalidateTimerHandle` _returnvalue))))

(fn `GetName`
  (returns (Name :type Text))
  (return "Spawner"))

(fn `UserConstructionScript`)