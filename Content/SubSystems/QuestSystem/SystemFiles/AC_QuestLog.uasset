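; Quest log component that holds the player's quests, spawning each as a BP_Quest_Base actor.
; Objective events are forwarded to every quest and refresh the tracked-quest HUD widget, while adding a quest credits collectibles already in inventory.
; Stage turn-in rebuilds nested quest structs, removes collected items using DT_Quests quantities, and grants XP, items and money through player subsystems.
; It also toggles quest tracking and the quest log UI.
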(event `self.ReceiveBeginPlay`
  (add `self.OnObjectiveCalled` (delegate `CheckObjective`)))

(event `CheckObjective` :!signature `self.OnObjectiveCalled`
  (params (ObjectiveID :type String))
  (bind _activequestuiref (`self.ActiveQuestUIRef`))
  (for _array_element (`self.CurrentQuests`)
    (`/Game/SubSystems/QuestSystem/SystemFiles/BP_Quest_Base.CheckObjective` _array_element ObjectiveID)
    (`/Engine/EditorBlueprintResources/StandardMacros.IsValid` _activequestuiref
      (:`Is Valid`
        (`/Game/SubSystems/QuestSystem/UI/WBP_ActiveQuest.RefreshInfo` _activequestuiref (`self.GetCurrentActiveQuest`))))))

(fn `AddQuest`
  (params (QuestID :type Name))
  (`KismetArrayLibrary.Array_AddUnique` (`self.AvailableQuests`) QuestID)
  (bind _returnvalue (`|SpawnActorFromClass` "/Game/SubSystems/QuestSystem/SystemFiles/BP_Quest_Base.BP_Quest_Base_C" (`KismetMathLibrary.MakeTransform` (0.0 0.0 0.0)) "Undefined" "OverrideRootScale" null QuestID null))
  (`KismetArrayLibrary.Array_Add` (`self.CurrentQuests`) _returnvalue)
  (bind _questdetails_questname (break `/Game/SubSystems/QuestSystem/SystemFiles/S_QuestDetails` (`/Game/SubSystems/QuestSystem/SystemFiles/BP_Quest_Base.QuestDetails` _returnvalue)))
  (`KismetSystemLibrary.PrintString` (`KismetStringLibrary.Concat_StrStr` "Quest " (`KismetTextLibrary.Conv_TextToString` _questdetails_questname) " spawned and added"))
  (`self.GetCollectionObjectives`))

(fn `CheckMoveToObjective`
  (params (ObjectiveID :type String))
  (locals (FoundObjectiveIndex :type Integer) (FoundStageIndex :type Integer) (FoundQuestIndex :type Integer) (FoundIndex :type Boolean) (FoundQuestStages :type "Array of /Game/SubSystems/QuestSystem/SystemFiles/S_QuestStage Structure") (FoundStageObjectives :type "Array of /Game/SubSystems/QuestSystem/SystemFiles/S_QuestObjective Structure"))
  (bind _output (`|GetArrayItem` (`self.CurrentQuests`) (`local.FoundQuestIndex`)))
  (bind (_questdetails_questname _questdetails_questlogdescription _questdetails_questshortdescription _questdetails_questtype _questdetails_queststages) (break `/Game/SubSystems/QuestSystem/SystemFiles/S_QuestDetails` (`/Game/SubSystems/QuestSystem/SystemFiles/BP_Quest_Base.QuestDetails` _output)))
  (bind (_questname _questlogdescription _questshortdescription _questtype) (break `/Game/SubSystems/QuestSystem/SystemFiles/S_QuestDetails` (`/Game/SubSystems/QuestSystem/SystemFiles/BP_Quest_Base.QuestDetails` _output)))
  (bind (_output_stagename _output_stagedescription _output_stageobjectives _output_xpreward _output_itemrewards _output_currencyreward _output_stagecomplete _output_stageturnedin) (break `/Game/SubSystems/QuestSystem/SystemFiles/S_QuestStage` (`|GetArrayItem` _questdetails_queststages (`local.FoundStageIndex`))))
  (bind (_objectivename _objectivedescription _objectivetype _objectiveid _quantity _isoptional _bonusxp) (break `/Game/SubSystems/QuestSystem/SystemFiles/S_QuestObjective` (`|GetArrayItem` _output_stageobjectives (`local.FoundObjectiveIndex`))))
  (bind _returnvalue (- _quantity 1))
  (bind _returnvalue_2 (<= _returnvalue 0))
  (for (_array_element _array_index) (`self.CurrentQuests`)
    (bind (_questdetails_questname_2 _questdetails_questlogdescription_2 _questdetails_questshortdescription_2 _questdetails_questtype_2 _questdetails_queststages_2) (break `/Game/SubSystems/QuestSystem/SystemFiles/S_QuestDetails` (`/Game/SubSystems/QuestSystem/SystemFiles/BP_Quest_Base.QuestDetails` _array_element)))
    (for _index (range (+ (`KismetArrayLibrary.Array_Length` _questdetails_queststages_2) 1))
      (bind (_output_stagename_2 _output_stagedescription_2 _output_stageobjectives_2 _output_xpreward_2 _output_itemrewards_2 _output_currencyreward_2 _output_stagecomplete_2) (break `/Game/SubSystems/QuestSystem/SystemFiles/S_QuestStage` (`|GetArrayItem` _questdetails_queststages_2 _index)))
      (if (not _output_stagecomplete_2)
        (for _index_2 (range (+ (`KismetArrayLibrary.Array_Length` _output_stageobjectives_2) 1))
          (if (== (`local.ObjectiveID`) (`.ObjectiveID_10_694D9AC5488D06DA773CAAA26F2403C1` (break `/Game/SubSystems/QuestSystem/SystemFiles/S_QuestObjective` (`|GetArrayItem` _output_stageobjectives_2 _index_2))))
            (set `local.FoundObjectiveIndex` _index_2)
            (set `local.FoundStageIndex` _index)
            (set `local.FoundQuestIndex` _array_index)
            (set `local.FoundIndex` true)
            (break)))
        (break)))
    (break))
  (if (`local.FoundIndex`)
    (`KismetSystemLibrary.PrintString` "Index found")
    (set `local.FoundQuestStages` _questdetails_queststages)
    (set `local.FoundStageObjectives` _output_stageobjectives)
    (if _returnvalue_2
      (`KismetSystemLibrary.PrintString` "LocationReached")
      (`KismetArrayLibrary.Array_Set` (`local.FoundStageObjectives`) (`local.FoundObjectiveIndex`) (make `/Game/SubSystems/QuestSystem/SystemFiles/S_QuestObjective` _objectivename _objectivedescription _objectivetype _objectiveid _returnvalue _isoptional _bonusxp (select `bool` _returnvalue_2 :`true` true)))
      (`KismetArrayLibrary.Array_Set` (`local.FoundQuestStages`) (`local.FoundStageIndex`) (make `/Game/SubSystems/QuestSystem/SystemFiles/S_QuestStage` _output_stagename _output_stagedescription (`local.FoundStageObjectives`) _output_xpreward _output_itemrewards _output_currencyreward _output_stagecomplete _output_stageturnedin))
      (set `/Game/SubSystems/QuestSystem/SystemFiles/BP_Quest_Base.QuestDetails` (make `/Game/SubSystems/QuestSystem/SystemFiles/S_QuestDetails` _questname _questlogdescription _questshortdescription _questtype (`local.FoundQuestStages`)) _output)
      (`KismetSystemLibrary.PrintString` "quest details updated"))
    (else
      (`KismetSystemLibrary.PrintString` "Index not found"))))

(fn `CompleteObjective`)

(fn `CompleteQuest`
  (params (QuestID :type Name))
  (if (`self.QueryActiveQuest` QuestID)
    (for _array_element (`self.CurrentQuests`)
      (if (== (`/Game/SubSystems/QuestSystem/SystemFiles/BP_Quest_Base.QuestID` _array_element) QuestID)
        (set `/Game/SubSystems/QuestSystem/SystemFiles/BP_Quest_Base.IsComplete` true _array_element)
        (`Actor.K2_DestroyActor` _array_element)))))

(fn `FindLocationObjective`
  (params (ObjectiveID :type String))
  (returns (ReturnValue :type Boolean))
  (bind _activequest (`self.GetCurrentActiveQuest`))
  (`/Engine/EditorBlueprintResources/StandardMacros.IsValid` _activequest
    (:`Is Valid`
      (bind _returnvalue (`/Game/SubSystems/QuestSystem/SystemFiles/BP_Quest_Base.FindStageForLocation` _activequest ObjectiveID))
      (return _returnvalue))
    (:`Is Not Valid`
      (return false))))

(fn `FindRequiredQuest`
  (params (QuestToFind :type Name))
  (returns (QuestIndexOut :type Integer) (QuestInstanceOut :type "/Game/SubSystems/QuestSystem/SystemFiles/BP_Quest_Base Object Reference"))
  (locals (QuestIndex :type Integer) (QuestInstance :type "/Game/SubSystems/QuestSystem/SystemFiles/BP_Quest_Base Object Reference"))
  (for (_array_element _array_index) (`self.CurrentQuests`)
    (if (== (`local.QuestToFind`) (`/Game/SubSystems/QuestSystem/SystemFiles/BP_Quest_Base.QuestID` _array_element))
      (set `local.QuestIndex` _array_index)
      (set `local.QuestInstance` _array_element)
      (break)))
  (return (`local.QuestIndex`) (`local.QuestInstance`)))

(fn `GetAmountForCollectionObjective`
  (params (StageIndex :type Integer) (ObjectiveIndex :type Integer) (QuestIndex :type Integer))
  (returns (Quantity :type Integer))
  (bind _returnvalue (`|GetDataTableRow` "/Game/SubSystems/QuestSystem/SystemFiles/DT_Quests.DT_Quests" (`/Game/SubSystems/QuestSystem/SystemFiles/BP_Quest_Base.QuestID` (`|GetArrayItem` (`self.CurrentQuests`) QuestIndex)))
    (:`then`
      (return (`.Quantity_13_8C8EF5EF40AFA90CA8EE609BB5B34FC6` (break `/Game/SubSystems/QuestSystem/SystemFiles/S_QuestObjective` (`|GetArrayItem` (`.StageObjectives_28_2D8A22E64FE3F94A518B81A2773BECCD` (break `/Game/SubSystems/QuestSystem/SystemFiles/S_QuestStage` (`|GetArrayItem` (`.QuestStages_15_BE0EEED04B7A83049F8879969C36533E` (break `/Game/SubSystems/QuestSystem/SystemFiles/S_QuestDetails` _returnvalue)) (`local.StageIndex`)))) (`local.ObjectiveIndex`))))))))

(fn `GetCollectionObjectives`
  (for _array_element (`self.CurrentQuests`)
    (for _array_element_2 (`.StageObjectives_28_2D8A22E64FE3F94A518B81A2773BECCD` (break `/Game/SubSystems/QuestSystem/SystemFiles/S_QuestStage` (`|GetArrayItem` (`.QuestStages_15_BE0EEED04B7A83049F8879969C36533E` (break `/Game/SubSystems/QuestSystem/SystemFiles/S_QuestDetails` (`/Game/SubSystems/QuestSystem/SystemFiles/BP_Quest_Base.QuestDetails` _array_element))) (`/Game/SubSystems/QuestSystem/SystemFiles/BP_Quest_Base.CurrentQuestStage` _array_element))))
      (bind (_objectivename _objectivedescription _objectivetype _objectiveid) (break `/Game/SubSystems/QuestSystem/SystemFiles/S_QuestObjective` _array_element_2))
      (if (`|EnumEquality` _objectivetype "NewEnumerator3")
        (bind (_success_ _totalamountininventory) (`/Game/SubSystems/Inventory/SystemFiles/AC_Inventory.FindItemInInventoryForObjective` (`/Game/Base/BFL_BasicFunctions.GetPlayerInventorySubsystem`) _objectiveid))
        (if _success_
          (for _ (range 1 (+ _totalamountininventory 1))
            (`/Game/SubSystems/QuestSystem/SystemFiles/BP_Quest_Base.CheckObjective` _array_element _objectiveid)))))))

(fn `GetCurrentActiveQuest`
  (returns (ActiveQuest :type "/Game/SubSystems/QuestSystem/SystemFiles/BP_Quest_Base Object Reference"))
  (locals (CurrentActiveQuest :type "/Game/SubSystems/QuestSystem/SystemFiles/BP_Quest_Base Object Reference") (`FoundQuest?` :type Boolean))
  (for _array_element (`self.CurrentQuests`)
    (if (== (`/Game/SubSystems/QuestSystem/SystemFiles/BP_Quest_Base.QuestID` _array_element) (`self.ActiveQuest`))
      (set `local.CurrentActiveQuest` _array_element)
      (set `local.FoundQuest?` true)
      (break)))
  (return (`local.CurrentActiveQuest`)))

(fn `OpenQuestLog`
  (bind _questloguiref (`self.QuestLogUIRef`)
    (:`then`
      (`Widget.RemoveFromParent` _questloguiref)
      (set `self.QuestLogUIRef` null))
    (:`else`
      (bind _returnvalue (`|CreateWidget` "/Game/SubSystems/QuestSystem/UI/WBP_QuestLogUI.WBP_QuestLogUI_C" null (`self.CurrentQuests`)))
      (bind _output_get (set `self.QuestLogUIRef` _returnvalue))
      (`UserWidget.AddToViewport` _output_get 0))))

(fn `QueryActiveQuest`
  (params (QuestID :type Name))
  (returns (ReturnValue :type Boolean))
  (return (`KismetArrayLibrary.Array_Contains` (`self.AvailableQuests`) QuestID)))

(fn `ReceiveStageRewards`
  (params (Stage :type "/Game/SubSystems/QuestSystem/SystemFiles/S_QuestStage Structure"))
  (locals (BonusExp :type Integer))
  (bind (_stagename _stagedescription _stageobjectives _xpreward _itemrewards _currencyreward _stagecomplete _stageturnedin) (break `/Game/SubSystems/QuestSystem/SystemFiles/S_QuestStage` Stage))
  (bind _playerinventory (`/Game/Base/BFL_BasicFunctions.GetPlayerInventorySubsystem`))
  (if (and _stagecomplete _stageturnedin)
    (for _array_element _stageobjectives
      (set `local.BonusExp` (+ (`.BonusXP_19_D74DD0B34BA25D457F8A0A9AEA751437` (break `/Game/SubSystems/QuestSystem/SystemFiles/S_QuestObjective` _array_element)) (`local.BonusExp`))))
    (`/Game/SubSystems/PlayerStats/SystemFiles/AC_CharacterStats.AddExperience` (`/Game/Base/BFL_BasicFunctions.GetPlayerStatsSubsystem`) (+ _xpreward (`local.BonusExp`)))
    (bind _keys (`BlueprintMapLibrary.Map_Keys` _itemrewards))
    (for _array_element_2 _keys
      (bind _returnvalue (`|GetDataTableRow` "/Game/SubSystems/Inventory/SystemFiles/DT_Items.DT_Items" _array_element_2)
        (:`then`
          (for _ (range 1 (+ (`BlueprintMapLibrary.Map_Find` _itemrewards _array_element_2) 1))
            (`/Game/SubSystems/Inventory/SystemFiles/AC_Inventory.AddToInventory` _playerinventory _returnvalue))
          (`/Game/SubSystems/Inventory/SystemFiles/AC_Inventory.AddMoney` _playerinventory _currencyreward))))))

(fn `TrackQuest`
  (params (QuestID :type Name))
  (bind _activequest (`self.GetCurrentActiveQuest`))
  (bind _activequestuiref (`self.ActiveQuestUIRef`))
  (if (== QuestID (`self.ActiveQuest`))
    (set `self.ActiveQuest` "None")
    (`/Engine/EditorBlueprintResources/StandardMacros.IsValid` _activequestuiref
      (:`Is Valid`
        (set `/Game/SubSystems/QuestSystem/UI/WBP_ActiveQuest.Active Quest` null _activequestuiref)
        (`/Engine/EditorBlueprintResources/StandardMacros.IsValid` _activequestuiref
          (:`Is Valid`
            (`Widget.RemoveFromParent` _activequestuiref)
            (set `self.ActiveQuestUIRef` null)))))
    (elif (`self.QueryActiveQuest` QuestID)
      (set `self.ActiveQuest` QuestID)
      (`/Engine/EditorBlueprintResources/StandardMacros.IsValid` _activequestuiref
        (:`Is Valid`
          (if (== _activequest (`/Game/SubSystems/QuestSystem/UI/WBP_ActiveQuest.Active Quest` _activequestuiref))
            (set `/Game/SubSystems/QuestSystem/UI/WBP_ActiveQuest.Active Quest` null _activequestuiref)
            (else
              (`/Game/SubSystems/QuestSystem/UI/WBP_ActiveQuest.RefreshInfo` _activequestuiref null))))
        (:`Is Not Valid`
          (bind _returnvalue (`|CreateWidget` "/Game/SubSystems/QuestSystem/UI/WBP_ActiveQuest.WBP_ActiveQuest_C" null _activequest))
          (bind _output_get (set `self.ActiveQuestUIRef` _returnvalue))
          (bind _returnvalue_2 (`CanvasPanel.AddChildToCanvas` (`/Game/Base/WBP_Player_UI.TrackedQuestCanvas` (`/Game/Base/BP_Player_HUD.PlayerUI_Ref` (`/Game/Base/BFL_BasicFunctions.Get Player HUD`))) _output_get))
          (`CanvasPanelSlot.SetAutoSize` _returnvalue_2 true))))))

(fn `TurnInStageQuest`
  (params (QuestIndex :type Integer) (StageIndex :type Integer))
  (returns (ReturnValue :type Integer) (Output_Get :type "/Game/SubSystems/QuestSystem/SystemFiles/S_QuestDetails Structure"))
  (locals (QuestStages :type "Array of /Game/SubSystems/QuestSystem/SystemFiles/S_QuestStage Structure"))
  (bind _playerinventory (`/Game/Base/BFL_BasicFunctions.GetPlayerInventorySubsystem`))
  (bind _queststages (`local.QuestStages`))
  (bind _stageindex (`local.StageIndex`))
  (bind _output (`|GetArrayItem` (`self.CurrentQuests`) QuestIndex))
  (bind (_stagename _stagedescription _stageobjectives _xpreward _itemrewards _currencyreward _stagecomplete) (break `/Game/SubSystems/QuestSystem/SystemFiles/S_QuestStage` (`|GetArrayItem` _queststages _stageindex)))
  (bind _questdetails (`/Game/SubSystems/QuestSystem/SystemFiles/BP_Quest_Base.QuestDetails` _output))
  (bind (_questname _questlogdescription _questshortdescription _questtype _queststages_2) (break `/Game/SubSystems/QuestSystem/SystemFiles/S_QuestDetails` _questdetails))
  (bind (_questname_2 _questlogdescription_2 _questshortdescription_2 _questtype_2) (break `/Game/SubSystems/QuestSystem/SystemFiles/S_QuestDetails` _questdetails))
  (bind _s_queststage (make `/Game/SubSystems/QuestSystem/SystemFiles/S_QuestStage` _stagename _stagedescription _stageobjectives _xpreward _itemrewards _currencyreward _stagecomplete true))
  (bind _returnvalue (`KismetArrayLibrary.Array_LastIndex` _queststages_2))
  (set `local.QuestStages` _queststages_2)
  (for (_array_element _array_index) (`.StageObjectives_28_2D8A22E64FE3F94A518B81A2773BECCD` (break `/Game/SubSystems/QuestSystem/SystemFiles/S_QuestStage` (`|GetArrayItem` _queststages_2 StageIndex)))
    (bind (_objectivename _objectivedescription _objectivetype _objectiveid) (break `/Game/SubSystems/QuestSystem/SystemFiles/S_QuestObjective` _array_element))
    (switch `/Game/SubSystems/QuestSystem/SystemFiles/E_QuestObjectiveType` _objectivetype
      (:`NewEnumerator0`
        (`KismetArrayLibrary.Array_Set` _queststages _stageindex _s_queststage :!label _label))
      (:`NewEnumerator2`
        (goto _label))
      (:`NewEnumerator3`
        (bind (_success_ _totalamountininventory _itemlookedforstruct) (`/Game/SubSystems/Inventory/SystemFiles/AC_Inventory.FindItemInInventoryForObjective` _playerinventory _objectiveid))
        (bind _quantity (`self.GetAmountForCollectionObjective` (`local.StageIndex`) _array_index (`local.QuestIndex`)))
        (for _ (range 1 (+ _quantity 1))
          (bind (_itemclass _itemname _itemdescription _itemtype _itemcurrentamount _itemstacksize _itemprice _equipmentinfo _aiditeminfo _icon _iteminventoryindex) (break `/Game/SubSystems/Inventory/SystemFiles/S_ItemInfo` _itemlookedforstruct))
          (`/Game/SubSystems/Inventory/SystemFiles/AC_Inventory.RemoveFromInventory` _playerinventory (make `/Game/SubSystems/Inventory/SystemFiles/S_ItemInfo` _itemclass _itemname _itemdescription _itemtype 1 _itemstacksize _itemprice _equipmentinfo _aiditeminfo _icon _iteminventoryindex))
          (goto _label)))))
  (`self.ReceiveStageRewards` _s_queststage)
  (bind _output_get (set `/Game/SubSystems/QuestSystem/SystemFiles/BP_Quest_Base.QuestDetails` (make `/Game/SubSystems/QuestSystem/SystemFiles/S_QuestDetails` _questname_2 _questlogdescription_2 _questshortdescription_2 _questtype_2 (`local.QuestStages`)) _output))
  (bind _result (`/Engine/EditorBlueprintResources/StandardMacros.IncrementInt` (`/Game/SubSystems/QuestSystem/SystemFiles/BP_Quest_Base.CurrentQuestStage` _output))
    (:`  `
      (return (select `bool` (> _result _returnvalue) :`false` _result :`true` _returnvalue) _output_get))))