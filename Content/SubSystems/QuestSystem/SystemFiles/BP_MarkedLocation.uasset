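; BP_MarkedLocation is a quest location marker that reports when the player reaches a location objective.
; Every tick it looks up its ObjectiveID in the player's quest log and shows its paper sprite in scene captures only while that objective is found.
; When a BP_Player overlaps its sphere, it passes the ObjectiveID to that player's QuestLogComponent as an objective call.
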(event `self.ReceiveTick`
  (params (DeltaSeconds :type "Float (single-precision)"))
  (bind _returnvalue (`/Game/SubSystems/QuestSystem/SystemFiles/AC_QuestLog.FindLocationObjective` (`/Game/Base/BFL_BasicFunctions.GetPlayerQuestLog`) (`self.ObjectiveID`)))
  (`PrimitiveComponent.SetHiddenInSceneCapture` (`self.PaperSprite`) (not _returnvalue)))

(event `self.Sphere.OnComponentBeginOverlap`
  (params (OverlappedComponent :type "PrimitiveComponent Object Reference") (OtherActor :type "Actor Object Reference") (OtherComp :type "PrimitiveComponent Object Reference") (OtherBodyIndex :type Integer) (bFromSweep :type Boolean) (SweepResult :type "HitResult Structure (by ref)"))
  (bind _asbp_player (cast `/Game/Base/BP_Player` OtherActor))
  (`/Game/SubSystems/QuestSystem/SystemFiles/AC_QuestLog.OnObjectiveCalled` (`/Game/Base/BP_Player.QuestLogComponent` _asbp_player) (`self.ObjectiveID`)))

(fn `UserConstructionScript`)