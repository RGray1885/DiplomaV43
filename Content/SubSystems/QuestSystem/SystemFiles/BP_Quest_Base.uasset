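; Base quest actor that loads its details from DT_Quests by QuestID at BeginPlay and tracks objective, stage and quest completion.
; CheckObjective decrements a matching current-stage objective's quantity, rebuilds the nested structs, then calls CheckStagesForCompletion, which completes stages based on non-optional objectives.
; CheckQuestForCompletion, not called here, sets IsComplete when all stages are complete.
; FindStageForLocation reports whether the current stage holds an objective ID not both completed and turned in.
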(event `self.ReceiveBeginPlay`
  (`self.SetQuestDetails`))

(fn `CheckObjective`
  (params (ObjectiveID :type String))
  (locals (QuestStages :type "Array of /Game/SubSystems/QuestSystem/SystemFiles/S_QuestStage Structure") (StageObjectives :type "Array of /Game/SubSystems/QuestSystem/SystemFiles/S_QuestObjective Structure") (FoundObjectiveIndex :type Integer))
  (bind _currentqueststage (`self.CurrentQuestStage`))
  (bind _stageobjectives (`local.StageObjectives`))
  (bind _stageobjectives_2 (`local.StageObjectives`))
  (bind _queststages (`local.QuestStages`))
  (bind _currentqueststage_2 (`self.CurrentQuestStage`))
  (bind (_questname _questlogdescription _questshortdescription _questtype) (break `/Game/SubSystems/QuestSystem/SystemFiles/S_QuestDetails` (`self.QuestDetails`)))
  (bind (_stagename _stagedescription _stageobjectives_3 _xpreward _itemrewards _currencyreward _stagecomplete _stageturnedin) (break `/Game/SubSystems/QuestSystem/SystemFiles/S_QuestStage` (`|GetArrayItem` _queststages _currentqueststage_2)))
  (bind _output_get (set `local.QuestStages` (`.QuestStages_15_BE0EEED04B7A83049F8879969C36533E` (break `/Game/SubSystems/QuestSystem/SystemFiles/S_QuestDetails` (`self.QuestDetails`)))))
  (set `local.StageObjectives` (`.StageObjectives_28_2D8A22E64FE3F94A518B81A2773BECCD` (break `/Game/SubSystems/QuestSystem/SystemFiles/S_QuestStage` (`|GetArrayItem` (`local.QuestStages`) _currentqueststage))))
  (if (<= _currentqueststage (`KismetArrayLibrary.Array_Length` _output_get))
    (for _index (range (+ (`KismetArrayLibrary.Array_Length` _stageobjectives) 1))
      (bind (_objectivename _objectivedescription _objectivetype _objectiveid _quantity _isoptional _bonusxp _objectivecomplete) (break `/Game/SubSystems/QuestSystem/SystemFiles/S_QuestObjective` (`|GetArrayItem` _stageobjectives _index)))
      (if (and (not _objectivecomplete) (== _objectiveid (`local.ObjectiveID`)))
        (bind _output_get_2 (set `local.FoundObjectiveIndex` _index))
        (bind (_objectivename_2 _objectivedescription_2 _objectivetype_2 _objectiveid_2 _quantity_2 _isoptional_2 _bonusxp_2) (break `/Game/SubSystems/QuestSystem/SystemFiles/S_QuestObjective` (`|GetArrayItem` _stageobjectives_2 _output_get_2)))
        (bind _returnvalue (- _quantity_2 1))
        (`KismetArrayLibrary.Array_Set` _stageobjectives_2 _output_get_2 (make `/Game/SubSystems/QuestSystem/SystemFiles/S_QuestObjective` _objectivename_2 _objectivedescription_2 _objectivetype_2 _objectiveid_2 _returnvalue _isoptional_2 _bonusxp_2 (select `bool` (<= _returnvalue 0) :`true` true)))
        (`KismetArrayLibrary.Array_Set` _queststages _currentqueststage_2 (make `/Game/SubSystems/QuestSystem/SystemFiles/S_QuestStage` _stagename _stagedescription (`local.StageObjectives`) _xpreward _itemrewards _currencyreward _stagecomplete _stageturnedin))
        (set `self.QuestDetails` (make `/Game/SubSystems/QuestSystem/SystemFiles/S_QuestDetails` _questname _questlogdescription _questshortdescription _questtype (`local.QuestStages`)))))
    (`self.CheckStagesForCompletion`)))

(fn `CheckQuestForCompletion`
  (locals (AllStagesComplete :type "Array of Boolean"))
  (bind _allstagescomplete (`local.AllStagesComplete`))
  (for _array_element (`.QuestStages_15_BE0EEED04B7A83049F8879969C36533E` (break `/Game/SubSystems/QuestSystem/SystemFiles/S_QuestDetails` (`self.QuestDetails`)))
    (`KismetArrayLibrary.Array_Add` _allstagescomplete (`.StageComplete_24_C95E3EA34241D54847207ABD5301287C` (break `/Game/SubSystems/QuestSystem/SystemFiles/S_QuestStage` _array_element))))
  (if (not (`KismetArrayLibrary.Array_Contains` _allstagescomplete))
    (`KismetSystemLibrary.PrintString` "AllStagesCompleted" true true (struct :`G` 0.201556 :`B` 0.056128 :`A` 1.0))
    (set `self.IsComplete` true)
    (`KismetSystemLibrary.PrintString` "QuestCompleted" true true (struct :`G` 0.203125 :`B` 0.05607 :`A` 1.0))))

(fn `CheckStagesForCompletion`
  (locals (QuestStages :type "Array of /Game/SubSystems/QuestSystem/SystemFiles/S_QuestStage Structure") (MainObjectivesComplete :type "Array of Boolean") (AllObjectivesComplete :type "Array of Boolean") (CompletedStageIndex :type Integer))
  (bind (_questname _questlogdescription _questshortdescription _questtype _queststages) (break `/Game/SubSystems/QuestSystem/SystemFiles/S_QuestDetails` (`self.QuestDetails`)))
  (bind (_questname_2 _questlogdescription_2 _questshortdescription_2 _questtype_2) (break `/Game/SubSystems/QuestSystem/SystemFiles/S_QuestDetails` (`self.QuestDetails`)))
  (bind _returnvalue (`KismetArrayLibrary.Array_Contains` (`local.AllObjectivesComplete`)))
  (bind _returnvalue_2 (`KismetArrayLibrary.Array_Contains` (`local.MainObjectivesComplete`)))
  (bind (_stagename _stagedescription _stageobjectives _xpreward _itemrewards _currencyreward _stagecomplete _stageturnedin) (break `/Game/SubSystems/QuestSystem/SystemFiles/S_QuestStage` (`|GetArrayItem` (`local.QuestStages`) (`local.CompletedStageIndex`))))
  (set `local.QuestStages` _queststages)
  (for (_array_element _array_index) _queststages
    (bind (_stagename_2 _stagedescription_2 _stageobjectives_2 _xpreward_2 _itemrewards_2 _currencyreward_2 _stagecomplete_2) (break `/Game/SubSystems/QuestSystem/SystemFiles/S_QuestStage` _array_element))
    (if (not _stagecomplete_2)
      (for _array_element_2 _stageobjectives_2
        (bind (_objectivename _objectivedescription _objectivetype _objectiveid _quantity _isoptional _bonusxp _objectivecomplete) (break `/Game/SubSystems/QuestSystem/SystemFiles/S_QuestObjective` _array_element_2))
        (if (not _isoptional)
          (`KismetArrayLibrary.Array_Add` (`local.MainObjectivesComplete`) _objectivecomplete))
        (`KismetArrayLibrary.Array_Add` (`local.AllObjectivesComplete`) _objectivecomplete))
      (`KismetSystemLibrary.PrintString` (`KismetMathLibrary.SelectString` "Not all objectives completed" "All objectives completed" _returnvalue))
      (if (not _returnvalue)
        (`KismetSystemLibrary.PrintString` (`KismetMathLibrary.SelectString` "Not all main objectives completed" "All main objectives completed" _returnvalue_2) :!label _label)
        (set `local.CompletedStageIndex` _array_index)
        (`KismetArrayLibrary.Array_Set` (`local.QuestStages`) (`local.CompletedStageIndex`) (make `/Game/SubSystems/QuestSystem/SystemFiles/S_QuestStage` _stagename _stagedescription _stageobjectives _xpreward _itemrewards _currencyreward true _stageturnedin))
        (set `self.QuestDetails` (make `/Game/SubSystems/QuestSystem/SystemFiles/S_QuestDetails` _questname_2 _questlogdescription_2 _questshortdescription_2 _questtype_2 (`local.QuestStages`)))
        (elif (not _returnvalue_2)
          (goto _label))))))

(fn `FindStageForLocation`
  (params (ObjectiveID :type String))
  (returns (ReturnValue :type Boolean))
  (locals (QuestStages :type "Array of /Game/SubSystems/QuestSystem/SystemFiles/S_QuestStage Structure") (StageObjectives :type "Array of /Game/SubSystems/QuestSystem/SystemFiles/S_QuestObjective Structure") (Found :type Boolean))
  (bind _currentqueststage (`self.CurrentQuestStage`))
  (bind _stageobjectives (`local.StageObjectives`))
  (bind (_stagename _stagedescription _stageobjectives_2 _xpreward _itemrewards _currencyreward _stagecomplete _stageturnedin) (break `/Game/SubSystems/QuestSystem/SystemFiles/S_QuestStage` (`|GetArrayItem` (`local.QuestStages`) _currentqueststage)))
  (bind _output_get (set `local.QuestStages` (`.QuestStages_15_BE0EEED04B7A83049F8879969C36533E` (break `/Game/SubSystems/QuestSystem/SystemFiles/S_QuestDetails` (`self.QuestDetails`)))))
  (set `local.StageObjectives` _stageobjectives_2)
  (if (<= _currentqueststage (`KismetArrayLibrary.Array_Length` _output_get))
    (for _index (range (+ (`KismetArrayLibrary.Array_Length` _stageobjectives) 1))
      (bind (_objectivename _objectivedescription _objectivetype _objectiveid _quantity _isoptional _bonusxp _objectivecomplete) (break `/Game/SubSystems/QuestSystem/SystemFiles/S_QuestObjective` (`|GetArrayItem` _stageobjectives _index)))
      (if (== (`local.ObjectiveID`) _objectiveid)
        (if (not (and _objectivecomplete _stageturnedin))
          (set `local.Found` true)
          (break))))
    (return (`local.Found`))))

(fn `SetQuestDetails`
  (bind _returnvalue (`|GetDataTableRow` "/Game/SubSystems/QuestSystem/SystemFiles/DT_Quests.DT_Quests" (`self.QuestID`))
    (:`then`
      (set `self.QuestDetails` _returnvalue))))

(fn `UserConstructionScript`)