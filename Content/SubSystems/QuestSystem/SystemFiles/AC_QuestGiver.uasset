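; Quest giver component that shows its assigned quest in the player's HUD.
; InteractWithQuestGiver calls DisplayQuest, printing a notice if the quest is already active, and returns the owner's name.
; DisplayQuest fills the QuestGiverCanvas with a WBP_QuestGiverUI, using the quest log's copy for active quests, otherwise the data table row.
; DisplayQuestForTurnIn, not called here, shows only the logged copy.
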(fn `DisplayQuest`
  (bind _questlogcomponent (`/Game/Base/BFL_BasicFunctions.GetPlayerQuestLog`))
  (bind (_questdata_datatable _questdata_rowname) (break `DataTableRowHandle` (`self.QuestData`)))
  (bind _returnvalue (`/Game/SubSystems/QuestSystem/SystemFiles/AC_QuestLog.QueryActiveQuest` _questlogcomponent _questdata_rowname))
  (bind _questgivercanvas (`/Game/Base/WBP_Player_UI.QuestGiverCanvas` (`/Game/Base/BP_Player_HUD.PlayerUI_Ref` (`/Game/Base/BFL_BasicFunctions.Get Player HUD`))))
  (`PanelWidget.ClearChildren` _questgivercanvas)
  (if (not _returnvalue)
    (bind _returnvalue_2 (`|GetDataTableRow` _questdata_datatable _questdata_rowname)
      (:`then`
        (bind _returnvalue_3 (`|CreateWidget` "/Game/SubSystems/QuestSystem/UI/WBP_QuestGiverUI.WBP_QuestGiverUI_C" null _questdata_rowname (select `bool` _returnvalue :`false` _returnvalue_2 :`true` (`/Game/SubSystems/QuestSystem/SystemFiles/BP_Quest_Base.QuestDetails` (stale _array_element))) :!label _label))
        (bind _returnvalue_4 (`CanvasPanel.AddChildToCanvas` _questgivercanvas _returnvalue_3))
        (`CanvasPanelSlot.SetAutoSize` _returnvalue_4 true)))
    (else
      (for _array_element (`/Game/SubSystems/QuestSystem/SystemFiles/AC_QuestLog.CurrentQuests` _questlogcomponent)
        (if (== _questdata_rowname (`/Game/SubSystems/QuestSystem/SystemFiles/BP_Quest_Base.QuestID` _array_element))
          (`PanelWidget.ClearChildren` _questgivercanvas)
          (goto _label))))))

(fn `DisplayQuestForTurnIn`
  (bind (_questdata_datatable _questdata_rowname) (break `DataTableRowHandle` (`self.QuestData`)))
  (bind _questgivercanvas (`/Game/Base/WBP_Player_UI.QuestGiverCanvas` (`/Game/Base/BP_Player_HUD.PlayerUI_Ref` (`/Game/Base/BFL_BasicFunctions.Get Player HUD`))))
  (bind _returnvalue (`|GetDataTableRow` _questdata_datatable _questdata_rowname)
    (:`then`
      (for _array_element (`/Game/SubSystems/QuestSystem/SystemFiles/AC_QuestLog.CurrentQuests` (`/Game/Base/BFL_BasicFunctions.GetPlayerQuestLog`))
        (bind _questid (`/Game/SubSystems/QuestSystem/SystemFiles/BP_Quest_Base.QuestID` _array_element))
        (if (== _questdata_rowname _questid)
          (`PanelWidget.ClearChildren` _questgivercanvas)
          (bind _returnvalue_2 (`|CreateWidget` "/Game/SubSystems/QuestSystem/UI/WBP_QuestGiverUI.WBP_QuestGiverUI_C" null _questid (`/Game/SubSystems/QuestSystem/SystemFiles/BP_Quest_Base.QuestDetails` _array_element)))
          (bind _returnvalue_3 (`CanvasPanel.AddChildToCanvas` _questgivercanvas _returnvalue_2))
          (`CanvasPanelSlot.SetAutoSize` _returnvalue_3 true))))))

(fn `InteractWithQuestGiver`
  (returns (ObjectiveID :type String))
  (bind (_questdata_datatable _questdata_rowname) (break `DataTableRowHandle` (`self.QuestData`)))
  (if (not (not (`/Game/SubSystems/QuestSystem/SystemFiles/AC_QuestLog.QueryActiveQuest` (`/Game/Base/BFL_BasicFunctions.GetPlayerQuestLog`) _questdata_rowname)))
    (`KismetSystemLibrary.PrintString` "Already have"))
  (`self.DisplayQuest`)
  (return (`KismetSystemLibrary.GetDisplayName` (`self.GetOwner`))))