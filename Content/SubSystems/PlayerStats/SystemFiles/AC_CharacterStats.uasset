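; Player stats component that holds attributes, health, mana, stamina, experience and levels.
; Attributes feed derived maximums, damage range and percentage-based Defense mitigation, while level-ups from a generated XP chart award attribute and ability points and refill health and mana.
; Stamina drains and regenerates through self-rescheduling timers tied to the running state.
; Changes broadcast EffectApplied or refresh the toggleable stats window; RestoreStamina and the health, mana and stamina Fortify functions only notify.
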(event `self.ReceiveBeginPlay`
  (`self.CalculateLevelChart`)
  (bind _asbp_player (cast `/Game/Base/BP_Player` (`self.GetOwner`)))
  (`self.CalculateBaseStats`)
  (set `self.HPCurrent` (/ (`self.HPMax`) 2.0))
  (set `self.ManaCurrent` (/ (`self.ManaMax`) 2.0))
  (set `self.StaminaCurrent` (`self.StaminaMax`)))

(fn `AddExperience`
  (params (ExpToAdd :type Integer))
  (locals (PreviousLevel :type Integer :default 0) (FoundIndex :type Integer) (bFoundIndex :type Boolean))
  (bind _levelchart (`self.LevelChart`))
  (bind _currentlevel (`self.CurrentLevel`))
  (bind _currentlevel_2 (`self.CurrentLevel`))
  (bind _foundindex (`local.FoundIndex`))
  (bind _returnvalue (- _foundindex 1))
  (set `local.PreviousLevel` _currentlevel_2)
  (if (not (>= _currentlevel_2 (`self.LevelCap`)))
    (bind _output_get (set `self.CurrentXP` (+ (`self.CurrentXP`) ExpToAdd)))
    (`self.EffectApplied`)
    (if (>= _output_get (`self.NextLevelXP`))
      (bind _keys (`BlueprintMapLibrary.Map_Keys` _levelchart))
      (`BlueprintMapLibrary.Map_Values` _levelchart)
      (for _array_element _keys
        (if (< (`self.CurrentXP`) (`BlueprintMapLibrary.Map_Find` _levelchart _array_element))
          (set `local.FoundIndex` _array_element)
          (set `local.bFoundIndex` true)
          (break)))
      (if (`local.bFoundIndex`)
        (set `self.NextLevelXP` (`BlueprintMapLibrary.Map_Find` _levelchart _foundindex))
        (bind _output_get_2 (set `self.CurrentLevel` (`KismetMathLibrary.SelectInt` _currentlevel _returnvalue (> _currentlevel _returnvalue))))
        (`self.OnLevelUp` (- _output_get_2 (`local.PreviousLevel`)))
        (bind _statswindowref (`self.StatsWindowRef`)
          (:`then`
            (`/Game/SubSystems/PlayerStats/UI/WBP_PlayerStats.Refresh` _statswindowref))
          (:`else`
            _))
        (if (>= (`self.CurrentLevel`) (`self.LevelCap`))
          (`KismetSystemLibrary.PrintString` "MaxLevel\\"))
        (else
          (`KismetSystemLibrary.PrintString` "Smth in \"Add Experience\" function is broken." true true (struct :`R` 1.0 :`A` 1.0)))))))

(fn `ApplyItemEffect`
  (params (ItemEffect :type "/Game/SubSystems/Inventory/SystemFiles/E_AidItemEffect Enum" :default "NewEnumerator0") (EffectPotency :type Integer) (EffectDuration :type "Float (double-precision)"))
  (locals (EffectTimer :type "TimerHandle Structure"))
  (switch `/Game/SubSystems/Inventory/SystemFiles/E_AidItemEffect` ItemEffect
    (:`NewEnumerator0`
      (`self.RestoreHealth` EffectPotency))
    (:`NewEnumerator1`
      (`self.RestoreMana` EffectPotency)))
  (`self.EffectApplied`)
  (bind _statswindowref (`self.StatsWindowRef`)
    (:`then`
      (`/Game/SubSystems/PlayerStats/UI/WBP_PlayerStats.StatsChanged` _statswindowref))
    (:`else`)))

(fn `CalculateBaseStats`
  (locals (FinalDamageBonus :type "Float (double-precision)" :default 0.0) (FinalDefenseBonus :type "Float (double-precision)" :default 0.0))
  (bind _vitality (`self.Vitality`))
  (bind _strength (`self.Strength`))
  (set `self.DamageMin` (`KismetMathLibrary.Conv_IntToDouble` (/ _strength 2)))
  (set `self.DamageMax` (`KismetMathLibrary.Conv_IntToDouble` _strength))
  (set `self.Defense` (`KismetMathLibrary.Conv_IntToDouble` (`self.Dexterity`)))
  (set `self.StaminaMax` (`KismetMathLibrary.Conv_IntToDouble` (* _vitality 20)))
  (set `self.HPMax` (`KismetMathLibrary.Conv_IntToDouble` (* _vitality 10)))
  (set `self.ManaMax` (`KismetMathLibrary.Conv_IntToDouble` (* (`self.Energy`) 10))))

(fn `CalculateLevelChart`
  (bind _levelchart (`self.LevelChart`))
  (for _index (range (+ (`self.LevelCap`) 1))
    (`BlueprintMapLibrary.Map_Add` (`self.LevelChart`) _index (* (/ (* _index (- _index 1)) 2) 1000)))
  (bind _keys (`BlueprintMapLibrary.Map_Keys` _levelchart))
  (bind _values (`BlueprintMapLibrary.Map_Values` _levelchart))
  (set `self.NextLevelXP` (`|GetArrayItem` _values (`|GetArrayItem` _keys (+ (`self.CurrentLevel`) 1))))
  (`KismetSystemLibrary.PrintString` (`KismetStringLibrary.Concat_StrStr` "Keys length " (`KismetStringLibrary.Conv_IntToString` (`KismetArrayLibrary.Array_Length` _keys)) "XP to max " (`KismetStringLibrary.Conv_IntToString` (`|GetArrayItem` _values (`|GetArrayItem` _keys (`self.LevelCap`)))))))

(fn `ChangeAbility`
  (params (AttributeName :type String) (`ShouldIncrease?` :type Boolean))
  (bind _strength (`self.Strength`))
  (bind _dexterity (`self.Dexterity`))
  (bind _vitality (`self.Vitality`))
  (bind _energy (`self.Energy`))
  (bind _returnvalue (`KismetMathLibrary.SelectInt` (+ _energy 1) (- _energy 1) `ShouldIncrease?`))
  (bind _returnvalue_2 (`KismetMathLibrary.SelectInt` (+ _strength 1) (- _strength 1) `ShouldIncrease?`))
  (bind _returnvalue_3 (`KismetMathLibrary.SelectInt` (+ _dexterity 1) (- _dexterity 1) `ShouldIncrease?`))
  (bind _returnvalue_4 (`KismetMathLibrary.SelectInt` (+ _vitality 1) (- _vitality 1) `ShouldIncrease?`))
  (switch `string` AttributeName
    (:`Strength`
      (if (< _returnvalue_2 1)
        (`KismetSystemLibrary.PrintString` "At minimum level, cannot be descreased further" :!label _label)
        (else
          (set `self.Strength` _returnvalue_2)
          (`/Engine/EditorBlueprintResources/StandardMacros.DecrementInt` (`self.AttributePoints`) :!label _label_2
            (:`  `
              (`self.EffectApplied`)
              (`self.CalculateBaseStats`)
              (if (< (`self.StaminaCurrent`) (`self.StaminaMax`))
                (`self.RegenStamina`)))))))
    (:`Dexterity`
      (if (< _returnvalue_3 1)
        (goto _label)
        (else
          (set `self.Dexterity` _returnvalue_3)
          (goto _label_2))))
    (:`Vitality`
      (if (< _returnvalue_4 1)
        (goto _label)
        (else
          (set `self.Vitality` _returnvalue_4)
          (goto _label_2))))
    (:`Energy`
      (if (< _returnvalue 1)
        (goto _label)
        (else
          (set `self.Energy` _returnvalue)
          (goto _label_2))))))

(fn `DamageHealth`
  (params (DamageAmount :type "Float (double-precision)"))
  (returns (IsHealthAtZero :type Boolean))
  (bind _returnvalue (- DamageAmount (* DamageAmount (* (`self.Defense`) 0.1))))
  (bind _output_get (set `self.HPCurrent` (`KismetMathLibrary.FClamp` (- (`self.HPCurrent`) (`KismetMathLibrary.SelectFloat` 0.0 _returnvalue (< _returnvalue 0.0))) 0.0 (`self.HPMax`))))
  (`self.EffectApplied`)
  (return (<= _output_get 0.0)))

(fn `DeFortifyDefence`
  (params (FortifyAmount :type "Float (double-precision)"))
  (bind _skilldefensebonus (`self.SkillDefenseBonus`))
  (set `self.SkillDefenseBonus` (`KismetMathLibrary.SelectFloat` 0.0 (- _skilldefensebonus FortifyAmount) (== _skilldefensebonus 0.0)))
  (`self.CalculateBaseStats`)
  (`self.EffectApplied`)
  (bind _statswindowref (`self.StatsWindowRef`)
    (:`then`
      (`/Game/SubSystems/PlayerStats/UI/WBP_PlayerStats.StatsChanged` _statswindowref))
    (:`else`)))

(fn `DrainMana`
  (params (AmountToDrain :type "Float (double-precision)"))
  (set `self.ManaCurrent` (- (`self.ManaCurrent`) AmountToDrain))
  (`self.EffectApplied`)
  (bind _statswindowref (`self.StatsWindowRef`)
    (:`then`
      (`/Game/SubSystems/PlayerStats/UI/WBP_PlayerStats.StatsChanged` _statswindowref))
    (:`else`)))

(fn `DrainStamina`
  (locals (DrainTimer :type "TimerHandle Structure"))
  (bind _playercharacter (`/Game/Base/BFL_BasicFunctions.GetPlayerCharacter`))
  (bind _staminacurrent (`self.StaminaCurrent`))
  (bind _isrunning (`/Game/Base/BP_Player.IsRunning` _playercharacter))
  (if _isrunning
    (if (<= _staminacurrent 0.0)
      (`KismetSystemLibrary.K2_ClearAndInvalidateTimerHandle` (`local.DrainTimer`) :!label _label)
      (`/Game/Base/BP_Player.Run` _playercharacter _isrunning)
      (else
        (`KismetSystemLibrary.PrintString` "DrainingStamina")
        (bind _output_get (set `self.StaminaCurrent` (`KismetMathLibrary.FClamp` (- _staminacurrent (`self.StaminaDrain`)) 0.0 (`self.StaminaMax`))))
        (`self.EffectApplied`)
        (if (<= _output_get 0.0)
          (goto _label)
          (else
            (bind _returnvalue (`KismetSystemLibrary.K2_SetTimer` null "DrainStamina" (`self.StaminaRegenRate`)))
            (set `local.DrainTimer` _returnvalue)))))
    (`self.EffectApplied`)
    (bind _statswindowref (`self.StatsWindowRef`)
      (:`then`
        (`/Game/SubSystems/PlayerStats/UI/WBP_PlayerStats.StatsChanged` _statswindowref))
      (:`else`))))

(fn `FortifyDefence`
  (params (FortifyAmount :type "Float (double-precision)"))
  (set `self.SkillDefenseBonus` (+ (`self.SkillDefenseBonus`) FortifyAmount))
  (`self.CalculateBaseStats`)
  (`self.EffectApplied`)
  (bind _statswindowref (`self.StatsWindowRef`)
    (:`then`
      (`/Game/SubSystems/PlayerStats/UI/WBP_PlayerStats.StatsChanged` _statswindowref))
    (:`else`)))

(fn `FortifyHealth`
  (params (EffectPotency :type Integer))
  (`self.EffectApplied`)
  (bind _statswindowref (`self.StatsWindowRef`)
    (:`then`
      (`/Game/SubSystems/PlayerStats/UI/WBP_PlayerStats.StatsChanged` _statswindowref))
    (:`else`)))

(fn `FortifyMana`
  (params (EffectPotency :type Integer))
  (`self.EffectApplied`)
  (bind _statswindowref (`self.StatsWindowRef`)
    (:`then`
      (`/Game/SubSystems/PlayerStats/UI/WBP_PlayerStats.StatsChanged` _statswindowref))
    (:`else`)))

(fn `FortifyStamina`
  (params (EffectPotency :type Integer))
  (`self.EffectApplied`)
  (bind _statswindowref (`self.StatsWindowRef`)
    (:`then`
      (`/Game/SubSystems/PlayerStats/UI/WBP_PlayerStats.StatsChanged` _statswindowref))
    (:`else`)))

(fn `OnLevelUp`
  (params (Times :type Integer))
  (set `self.AttributePoints` (+ (`self.AttributePoints`) (* Times 3)))
  (set `self.AbilityPoints` (+ (`self.AbilityPoints`) Times))
  (set `self.ManaCurrent` (`self.ManaMax`))
  (set `self.HPCurrent` (`self.HPMax`))
  (`self.EffectApplied`)
  (bind _statswindowref (`self.StatsWindowRef`)
    (:`then`
      (`/Game/SubSystems/PlayerStats/UI/WBP_PlayerStats.StatsChanged` _statswindowref))
    (:`else`)))

(fn `OpenStatsScreen`
  (bind _statswindowref (`self.StatsWindowRef`)
    (:`then`
      (`Widget.RemoveFromParent` _statswindowref)
      (set `self.StatsWindowRef` null))
    (:`else`
      (bind _returnvalue (`|CreateWidget` "/Game/SubSystems/PlayerStats/UI/WBP_PlayerStats.WBP_PlayerStats_C" null self))
      (bind _output_get (set `self.StatsWindowRef` _returnvalue))
      (bind _returnvalue_2 (`CanvasPanel.AddChildToCanvas` (`/Game/Base/WBP_Player_UI.StatsCanvas` (`/Game/Base/BP_Player_HUD.PlayerUI_Ref` (`/Game/Base/BFL_BasicFunctions.Get Player HUD`))) _output_get))
      (`CanvasPanelSlot.SetAutoSize` _returnvalue_2 true))))

(fn `RegenStamina`
  (locals (StaminaRegenTimer :type "TimerHandle Structure"))
  (if (not (`/Game/Base/BP_Player.IsRunning` (`/Game/Base/BFL_BasicFunctions.GetPlayerCharacter`)))
    (`KismetSystemLibrary.PrintString` "RegenStarted")
    (set `self.StaminaCurrent` (`KismetMathLibrary.FClamp` (+ (`self.StaminaCurrent`) (`self.StaminaRegenAmount`)) 0.0 (`self.StaminaMax`)))
    (if (>= (`self.StaminaCurrent`) (`self.StaminaMax`))
      (`KismetSystemLibrary.K2_ClearAndInvalidateTimerHandle` (`local.StaminaRegenTimer`))
      (else
        (bind _returnvalue (`KismetSystemLibrary.K2_SetTimer` null "RegenStamina" (`self.StaminaRegenRate`)))
        (set `local.StaminaRegenTimer` _returnvalue)))
    (`self.EffectApplied`)
    (bind _statswindowref (`self.StatsWindowRef`)
      (:`then`
        (`/Game/SubSystems/PlayerStats/UI/WBP_PlayerStats.StatsChanged` _statswindowref))
      (:`else`))))

(fn `RestoreHealth`
  (params (EffectPotency :type Integer))
  (bind _hpcurrent (`self.HPCurrent`))
  (set `self.HPCurrent` (`KismetMathLibrary.FClamp` (+ (`KismetMathLibrary.Conv_IntToDouble` EffectPotency) _hpcurrent) _hpcurrent (`self.HPMax`)))
  (`self.EffectApplied`)
  (bind _statswindowref (`self.StatsWindowRef`)
    (:`then`
      (`/Game/SubSystems/PlayerStats/UI/WBP_PlayerStats.StatsChanged` _statswindowref))
    (:`else`)))

(fn `RestoreMana`
  (params (EffectPotency :type Integer))
  (bind _manacurrent (`self.ManaCurrent`))
  (set `self.ManaCurrent` (`KismetMathLibrary.FClamp` (+ (`KismetMathLibrary.Conv_IntToDouble` EffectPotency) _manacurrent) _manacurrent (`self.ManaMax`)))
  (`self.EffectApplied`)
  (bind _statswindowref (`self.StatsWindowRef`)
    (:`then`
      (`/Game/SubSystems/PlayerStats/UI/WBP_PlayerStats.StatsChanged` _statswindowref))
    (:`else`)))

(fn `RestoreStamina`
  (params (EffectPotency :type Integer))
  (`self.EffectApplied`)
  (bind _statswindowref (`self.StatsWindowRef`)
    (:`then`
      (`/Game/SubSystems/PlayerStats/UI/WBP_PlayerStats.StatsChanged` _statswindowref))
    (:`else`)))