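; Player controller that turns input into actions on the player character.
; Movement follows the control rotation's yaw, while look axes scale by turn rate and frame time.
; Zoom adjusts the character's spring arm length within clamped limits.
; Jump, sprint, walk/run toggle, interact and melee attack forward to the character or its combat component, and the I key opens the inventory through the player inventory subsystem.
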(event `InputAxis|MoveForward`
  (params (AxisValue :type "Float (single-precision)"))
  (`Pawn.AddMovementInput` (`/Game/Base/BFL_BasicFunctions.GetPlayerCharacter`) (`KismetMathLibrary.GetForwardVector` (`KismetMathLibrary.MakeRotator` 0.0 0.0 (.yaw (`self.GetControlRotation`)))) AxisValue false))

(event `InputAxis|MoveRight`
  (params (AxisValue :type "Float (single-precision)"))
  (`Pawn.AddMovementInput` (`/Game/Base/BFL_BasicFunctions.GetPlayerCharacter`) (`KismetMathLibrary.GetRightVector` (`KismetMathLibrary.MakeRotator` 0.0 0.0 (.yaw (`self.GetControlRotation`)))) AxisValue false))

(event `InputAxis|Turn`
  (params (AxisValue :type "Float (single-precision)"))
  (`self.AddYawInput` (* AxisValue (`self.BaseTurnRate`) (`GameplayStatics.GetWorldDeltaSeconds`))))

(event `InputAxis|LookUp`
  (params (AxisValue :type "Float (single-precision)"))
  (`self.AddPitchInput` (* AxisValue (`self.BaseTurnRate`) (`GameplayStatics.GetWorldDeltaSeconds`))))

(event `InputAction|Jump`
  (params (Key :type "Key Structure"))
  (bind _playercharacter (`/Game/Base/BFL_BasicFunctions.GetPlayerCharacter`))
  (:`Pressed`
    (`Character.Jump` _playercharacter))
  (:`Released`
    (`Character.StopJumping` _playercharacter)))

(event `InputAxis|ZoomCamera`
  (params (AxisValue :type "Float (single-precision)"))
  (bind _springarm (`/Game/Base/BP_Player.SpringArm` (`/Game/Base/BFL_BasicFunctions.GetPlayerCharacter`)))
  (set `SpringArmComponent.TargetArmLength` (`KismetMathLibrary.FClamp` (+ (`SpringArmComponent.TargetArmLength` _springarm) (* AxisValue (`self.ZoomRate`))) 150.0 1000.0) _springarm))

(event `InputAction|Interact`
  (params (Key :type "Key Structure"))
  (:`Pressed`
    (`/Game/Base/BP_Player.Interact` (`/Game/Base/BFL_BasicFunctions.GetPlayerCharacter`))))

(event `InputAction|Sprint`
  (params (Key :type "Key Structure"))
  (bind _playercharacter (`/Game/Base/BFL_BasicFunctions.GetPlayerCharacter`))
  (:`Pressed`
    (`/Game/Base/BP_Player.Run` _playercharacter true))
  (:`Released`
    (`/Game/Base/BP_Player.Run` _playercharacter false)))

(event `InputAction|Toggle Walk/Run`
  (params (Key :type "Key Structure"))
  (:`Pressed`
    (`/Game/Base/BP_Player.SetMaxWalkSpeed` (`/Game/Base/BFL_BasicFunctions.GetPlayerCharacter`))))

(event `InputAction|Attack`
  (params (Key :type "Key Structure"))
  (:`Pressed`
    (`/Game/SubSystems/Combat/AC_CombatSystem.MeleeAttack` (`/Game/Base/BP_Player.CombatSystemComponent` (`/Game/Base/BFL_BasicFunctions.GetPlayerCharacter`)))))

(event `Key|I`
  (params (Key :type "Key Structure"))
  (:`Pressed`
    (`/Game/SubSystems/Inventory/SystemFiles/AC_Inventory.OpenInventoryScreen` (`/Game/Base/BFL_BasicFunctions.GetPlayerInventorySubsystem`))))

(fn `UserConstructionScript`)