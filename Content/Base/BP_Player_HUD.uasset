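; Player HUD Blueprint that creates the main player UI on BeginPlay and manages enemy target bars and a dialogue window within it.
; ShowTargetName replaces any current bar with a new one for the enemy actor on the UI's enemy canvas, removing it after a short retriggerable delay.
; ShowDialogueWindow toggles a mode-selection widget for the clicked actor, switching mouse cursor visibility and input mode accordingly.
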(event `self.ReceiveBeginPlay`
  (bind _returnvalue (`|CreateWidget` "/Game/Base/WBP_Player_UI.WBP_Player_UI_C"))
  (bind _output_get (set `self.PlayerUI_Ref` _returnvalue))
  (`UserWidget.AddToViewport` _output_get 0))

(event `ShowTargetName`
  (params (Actor :type "/Game/NPC/BP_NPC_Base Object Reference"))
  (bind _playerui_ref (`self.PlayerUI_Ref`)
    (:`then`
      (if (`/Game/NPC/BP_NPC_Base.IsEnemy` Actor)
        (`self.NPC_BarRef`
          (:`then`
            (`Widget.RemoveFromParent` (`self.NPC_BarRef`))
            (set `self.NPC_BarRef` null))
          (:`else`
            _))
        (bind _returnvalue (`|CreateWidget` "/Game/Base/WBP_EnemyBar.WBP_EnemyBar_C" null Actor))
        (bind _output_get (set `self.NPC_BarRef` _returnvalue))
        (bind _returnvalue_2 (`CanvasPanel.AddChildToCanvas` (`/Game/Base/WBP_Player_UI.EnemyCanvas` _playerui_ref) _output_get))
        (`CanvasPanelSlot.SetAutoSize` _returnvalue_2 true)
        (`KismetSystemLibrary.RetriggerableDelay` 2.0)
        (`Widget.RemoveFromParent` (`self.NPC_BarRef`))
        (set `self.NPC_BarRef` null)))
    (:`else`)))

(fn `ShowDialogueWindow`
  (params (ActorClickedOn :type "Actor Object Reference"))
  (bind _player_controller (`/Game/Base/BFL_BasicFunctions.GetPlayerController`))
  (bind _dialoguescreenref (`self.DialogueScreenRef`)
    (:`then`
      (`Widget.RemoveFromParent` _dialoguescreenref)
      (set `self.DialogueScreenRef` null)
      (set `PlayerController.bShowMouseCursor` false _player_controller)
      (`WidgetBlueprintLibrary.SetInputMode_GameOnly` _player_controller))
    (:`else`
      (bind _returnvalue (`|CreateWidget` "/Game/SubSystems/WBP_ModeSelection.WBP_ModeSelection_C" null ActorClickedOn))
      (bind _output_get (set `self.DialogueScreenRef` _returnvalue))
      (bind _returnvalue_2 (`CanvasPanel.AddChildToCanvas` (`/Game/Base/WBP_Player_UI.ModeSelectionCanvas` (`self.PlayerUI_Ref`)) _output_get))
      (`CanvasPanelSlot.SetAutoSize` _returnvalue_2 true)
      (set `PlayerController.bShowMouseCursor` true _player_controller)
      (`WidgetBlueprintLibrary.SetInputMode_GameAndUIEx` _player_controller null))))

(fn `UserConstructionScript`)