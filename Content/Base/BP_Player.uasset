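; BP_Player is the player character, handling movement speeds, stamina-limited running, damage and death, and interaction.
; PlayerStats tracks health and stamina: damage can trigger a death montage with input disabled, and running drains stamina.
; An InteractionRadius overlap fills ItemsInRange and shows friendly NPC widgets; Interact sends InteractMessage only to camera-traced actors in that list.
; MeleeAttack is empty, leaving the equipment-based montage combo logic disconnected.
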(event `self.ReceiveBeginPlay`
  (set `self.DefaultMaxSpeed` (`CharacterMovementComponent.MaxWalkSpeed` (`self.CharacterMovement`))))

(event `self.ReceiveAnyDamage`
  (params (Damage :type "Float (single-precision)") (DamageType :type "DamageType Object Reference") (InstigatedBy :type "Controller Object Reference") (DamageCauser :type "Actor Object Reference"))
  (`KismetSystemLibrary.RetriggerableDelay` 0.1)
  (if (<= (`/Game/SubSystems/PlayerStats/SystemFiles/AC_CharacterStats.HPCurrent` (`self.PlayerStats`)) 0.0)
    _
    (elif (not (== DamageCauser self))
      (bind _ishealthatzero (`/Game/SubSystems/PlayerStats/SystemFiles/AC_CharacterStats.DamageHealth` (`self.PlayerStats`) Damage))
      (if _ishealthatzero
        (`KismetSystemLibrary.PrintString` "Dead")
        (`self.PlayDead`)))))

(event `self.InteractionRadius.OnComponentBeginOverlap`
  (params (OverlappedComponent :type "PrimitiveComponent Object Reference") (OtherActor :type "Actor Object Reference") (OtherComp :type "PrimitiveComponent Object Reference") (OtherBodyIndex :type Integer) (bFromSweep :type Boolean) (SweepResult :type "HitResult Structure (by ref)"))
  (bind _itemsinrange (`self.ItemsInRange`))
  (castclass `/Game/SubSystems/Inventory/Equipment/BP_EquipmentBasic` (`GameplayStatics.GetObjectClass` OtherActor)
    (:`CastFailed`
      (if (not (`KismetArrayLibrary.Array_Contains` _itemsinrange OtherActor))
        (`KismetArrayLibrary.Array_Add` _itemsinrange OtherActor)
        (`KismetSystemLibrary.PrintString` (`KismetStringLibrary.BuildString_Object` "object " "" OtherActor " added"))
        (bind _asbp_npc_base (cast `/Game/NPC/BP_NPC_Base` OtherActor))
        (if (not (`/Game/NPC/BP_NPC_Base.IsEnemy` _asbp_npc_base))
          (`SceneComponent.SetHiddenInGame` (`/Game/NPC/BP_NPC_Base.Widget` _asbp_npc_base) false false))))))

(event `PlayDead`
  (bind _player_controller (`/Game/Base/BFL_BasicFunctions.GetPlayerController`))
  (bind _returnvalue (`SkeletalMeshComponent.GetAnimInstance` (`self.Mesh`)))
  (`MovementComponent.StopMovementImmediately` (`self.CharacterMovement`))
  (`self.DisableInput` _player_controller _player_controller)
  (`AnimInstance.Montage_Stop` _returnvalue 0.0 null)
  (`AnimInstance.Montage_Play` _returnvalue (`self.DeathMontage`) 1.0 "MontageLength" 0.0 true))

(event `self.InteractionRadius.OnComponentEndOverlap`
  (params (OverlappedComponent :type "PrimitiveComponent Object Reference") (OtherActor :type "Actor Object Reference") (OtherComp :type "PrimitiveComponent Object Reference") (OtherBodyIndex :type Integer))
  (bind _itemsinrange (`self.ItemsInRange`))
  (if (`KismetArrayLibrary.Array_Contains` _itemsinrange OtherActor)
    (`KismetArrayLibrary.Array_RemoveItem` _itemsinrange OtherActor)
    (`KismetSystemLibrary.PrintString` (`KismetStringLibrary.BuildString_Object` "object " "" OtherActor " removed"))
    (bind _asbp_npc_base (cast `/Game/NPC/BP_NPC_Base` OtherActor))
    (if (not (`/Game/NPC/BP_NPC_Base.IsEnemy` _asbp_npc_base))
      (`SceneComponent.SetHiddenInGame` (`/Game/NPC/BP_NPC_Base.Widget` _asbp_npc_base) true false))))

(event `SetMaxWalkSpeed`
  (bind _walkspeed (`self.WalkSpeed`))
  (bind _charactermovement (`self.CharacterMovement`))
  (bind _runspeed (`self.RunSpeed`))
  (`/Engine/EditorBlueprintResources/StandardMacros.FlipFlop`
    (:`A`
      (`|ExecutionSequence`
        (:`then_0`
          (set `CharacterMovementComponent.MaxWalkSpeed` _walkspeed _charactermovement))
        (:`then_1`
          (set `CharacterMovementComponent.MaxWalkSpeedCrouched` (/ _walkspeed 2.0) _charactermovement))))
    (:`B`
      (`|ExecutionSequence`
        (:`then_0`
          (set `CharacterMovementComponent.MaxWalkSpeed` _runspeed _charactermovement))
        (:`then_1`
          (set `CharacterMovementComponent.MaxWalkSpeedCrouched` (/ _runspeed 2.0) _charactermovement))))))

(event `MeleeAttack`)

(fn `Interact`
  (bind _returnvalue (`GameplayStatics.GetPlayerCameraManager` 0))
  (bind _returnvalue_2 (`self.K2_GetActorLocation` _returnvalue))
  (bind _outhit (`KismetSystemLibrary.LineTraceSingle` :`Start` _returnvalue_2 :`End` (+ _returnvalue_2 (* (`self.GetActorForwardVector` _returnvalue) (`self.TraceLength`))) :`TraceChannel` "TraceTypeQuery1" :`DrawDebugType` "ForDuration"))
  (bind (_bblockinghit _binitialoverlap _time _distance _location _impactpoint _normal _impactnormal _physmat _hitactor) (`GameplayStatics.BreakHitResult` _outhit))
  (if (`KismetArrayLibrary.Array_Contains` (`self.ItemsInRange`) _hitactor)
    (message `/Game/Base/BPI_Interact.Interact` _hitactor)))

(fn `QueryItemInRange`
  (params (Actor :type "Actor Object Reference"))
  (returns (ReturnValue :type Boolean))
  (return (`KismetArrayLibrary.Array_Contains` (`self.ItemsInRange`) Actor)))

(fn `Run`
  (params (`ShouldRun?` :type Boolean))
  (locals (DrainTimer :type "TimerHandle Structure") (TimerLoop :type Boolean) (RegenTimer :type "TimerHandle Structure"))
  (bind _charactermovement (`self.CharacterMovement`))
  (if (> (`KismetMathLibrary.VSize` (`self.GetVelocity`)) 0.0)
    (bind _output_get (set `self.IsRunning` `ShouldRun?`))
    (if _output_get
      (if (<= (`/Game/SubSystems/PlayerStats/SystemFiles/AC_CharacterStats.StaminaCurrent` (`self.PlayerStats`)) 0.0)
        (set `CharacterMovementComponent.MaxWalkSpeed` (`self.DefaultMaxSpeed`) _charactermovement :!label _label)
        (if (not (`self.IsRunning`))
          (`/Game/SubSystems/PlayerStats/SystemFiles/AC_CharacterStats.RegenStamina` (`self.PlayerStats`)))
        (else
          (set `CharacterMovementComponent.MaxWalkSpeed` (* (`self.DefaultMaxSpeed`) 2.0) _charactermovement)
          (`/Game/SubSystems/PlayerStats/SystemFiles/AC_CharacterStats.DrainStamina` (`self.PlayerStats`))))
      (else
        (goto _label)))))

(fn `UserConstructionScript`)